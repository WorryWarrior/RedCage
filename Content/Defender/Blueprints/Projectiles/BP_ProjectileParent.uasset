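; Parent projectile Blueprint that handles bullet impacts and damage when its collision sphere hits something.
; PhysicMatComp maps the hit physical material to an attached particle, decal, sound and damage multiplier, with decal fade screen size lowered to prevent fading.
; It applies point damage, pushes physics-simulating actors, fires a radial impulse for valid actors, then destroys itself.
; Hits without a valid physical material are ignored.
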(event `self.SphereCollision.OnComponentHit`
  (params (HitComponent :type "PrimitiveComponent Object Reference") (OtherActor :type "Actor Object Reference") (OtherComp :type "PrimitiveComponent Object Reference") (NormalImpulse :type "Vector Structure") (Hit :type "HitResult Structure (by ref)"))
  (bind (_bblockinghit _binitialoverlap _time _distance _location _impactpoint _normal _impactnormal) (`GameplayStatics.BreakHitResult` (`self.Hit`)))
  (set `self.Other` OtherActor)
  (set `self.Other Comp` OtherComp)
  (set `self.Hit` Hit)
  (set `self.Phys Mat` (`.PhysMat` (`GameplayStatics.BreakHitResult` (`self.Hit`))))
  (`self.Phys Mat`
    (:`then`
      (`self.SpawnParticle`)
      (bind _returnvalue (`GameplayStatics.SpawnDecalAttached` (`/Game/Defender/Blueprints/Components/PhysicMatComp.GetDecal` (`self.PhysicMatComp`) (`self.Phys Mat`)) (4.0 4.0 12.0) (`self.Other Comp`) (`.HitBoneName` (`GameplayStatics.BreakHitResult` (`self.Hit`))) _impactpoint (`KismetMathLibrary.MakeRotFromZ` _impactnormal) "KeepWorldPosition" 30.0)) ; Spawn decal on surface when bullet hit
      (`self.DecalSetFadeScreenSize` _returnvalue) ; Prevent fading decals
      (`GameplayStatics.PlaySoundAtLocation` (`/Game/Defender/Blueprints/Components/PhysicMatComp.GetBulletSound` (`self.PhysicMatComp`) (`self.Phys Mat`)) (`.ImpactPoint` (`GameplayStatics.BreakHitResult` (`self.Hit`))) (struct) 1.0 1.0 0.0 "/Game/Defender/Demo/Audio/Attenuations/ATT_BulletImpacts.ATT_BulletImpacts" "/Game/Defender/Demo/Audio/Concurrencies/Con_BulletImpactSound.Con_BulletImpactSound" null null)
      (set `self.HitFromDirection` (`KismetMathLibrary.GetForwardVector` (`self.K2_GetActorRotation`)))
      (`GameplayStatics.ApplyPointDamage` (`self.Other`) (* (`/Game/Defender/Blueprints/Components/PhysicMatComp.GetDamageMultiplier` (`self.PhysicMatComp`) (`self.Phys Mat`) (`self.Vulnarable Damage Multiplier`)) (`self.Damage`)) (`self.HitFromDirection`) (`self.Hit`) (`GameplayStatics.GetPlayerController` 0) self "/Script/Engine.DamageType") ; Apply point damage to hit actor
      (`self.AddImpulseToOther`)
      (`self.K2_DestroyActor`))
    (:`else`)))

(event `AddImpulseToOther`
  (`/Engine/EditorBlueprintResources/StandardMacros.IsValid` (`self.Other`)
    (:`Is Valid`
      (if (`SceneComponent.IsSimulatingPhysics` (`Actor.RootComponent` (`self.Other`)) "None")
        (`PrimitiveComponent.AddImpulse` (cast `PrimitiveComponent` (`Actor.RootComponent` (`self.Other`)) :!pure true) (* (`self.HitFromDirection`) 20000.0) "None" false) ; Add impulse if hit actor is simulating physics
      )
      (`RadialForceComponent.FireImpulse` (`self.RadialForce`)) ; Fire radial impulse as well
    )))

(fn `DecalSetFadeScreenSize`
  (params (Decal :type "DecalComponent Object Reference"))
  (`/Engine/EditorBlueprintResources/StandardMacros.IsValid` Decal
    (:`Is Valid`
      (`DecalComponent.SetFadeScreenSize` Decal 0.005) ; Prevent fading decals
    )))

(fn `PhysicMatDetermination`
  (locals (Particle :type "ParticleSystem Object Reference") (ParticleScale :type "Vector Structure" :default (1.0 1.0 1.0)) (PhysicMat :type "PhysicalMaterial Object Reference") (DecalMat :type "Material Object Reference" :default null))
  (bind _output_get (set `local.PhysicMat` (`.PhysMat` (`GameplayStatics.BreakHitResult` (`self.Hit`)))))
  (switch `EPhysicalSurface` (`PhysicalMaterial.SurfaceType` _output_get)
    (:`SurfaceType_Default`
      (set `local.Particle` "/Game/Defender/Demo/Particles/P_Impact.P_Impact")
      (set `local.ParticleScale` (0.3 0.3 0.3))
      (set `local.DecalMat` "/Engine/MaterialTemplates/VertexAnimation/AdvancedFlag.AdvancedFlag"))))

(fn `SpawnParticle`
  (locals (HitRot :type "Rotator Structure" :default (struct)))
  (bind (_particle _scale) (`/Game/Defender/Blueprints/Components/PhysicMatComp.GetParticleEffect` (`self.PhysicMatComp`) (`self.Phys Mat`)))
  (bind (_bblockinghit _binitialoverlap _time _distance _location _impactpoint _normal _impactnormal _physmat _hitactor _hitcomponent _hitbonename) (`GameplayStatics.BreakHitResult` (`self.Hit`)))
  (set `self.Hit Component` (`.HitComponent` (`GameplayStatics.BreakHitResult` (`self.Hit`))))
  (set `local.HitRot` (`KismetMathLibrary.MakeRotFromZ` (`.ImpactNormal` (`GameplayStatics.BreakHitResult` (`self.Hit`)))))
  (`GameplayStatics.SpawnEmitterAttached` _particle (`self.Hit Component`) _hitbonename _location (`local.HitRot`) _scale "KeepWorldPosition" true "AutoRelease"))

(fn `UserConstructionScript`)