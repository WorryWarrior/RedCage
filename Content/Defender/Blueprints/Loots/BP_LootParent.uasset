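; Base Blueprint for loot pickups that are thrown with random yaw and speed on spawn, then fly to the player to be collected.
; After a short pickup delay, overlapping the player enables Tick, which interpolates the loot toward them until close, with a timer fallback.
; Medkit and grenade subclasses are checked against inventory capacity.
; On pickup it plays a sound and passes its class to the player's LootComp, then destroys itself.
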(event `DelayedPickUpEvent`
  (set `self.CanBePickedUp` true) ; Loot can be picked after 1 second
)

(event `self.ReceiveBeginPlay`
  (bind (_returnvalue_roll _returnvalue_pitch _returnvalue_yaw) (`KismetMathLibrary.BreakRotator` (`KismetMathLibrary.RandomRotator` false)))
  (set `self.PlayerChar` (`GameplayStatics.GetPlayerCharacter` 0))
  (`KismetSystemLibrary.K2_SetTimerDelegate` (delegate `DelayedPickUpEvent`) 1.0)
  (`self.K2_SetActorRotation` (`KismetMathLibrary.MakeRotator` 0.0 100.0 _returnvalue_yaw))
  (set `ProjectileMovementComponent.InitialSpeed` (`KismetMathLibrary.RandomFloatInRange` 100.0 1500.0) (`self.ProjectileMovement`))
  (`KismetSystemLibrary.Delay` 0.2)
  (`self.ActivateProjectileMovement`) ; Activate Projectile Movement \nto throwing the loot
  ;[1 1 1] Check if loot is already overlapping
  (if (`self.IsOverlappingActor` (`self.PlayerChar`))
    (`KismetSystemLibrary.Delay` 1.0)
    (`self.StartToMoveChar`)))

(event `self.Sphere.OnComponentBeginOverlap`
  (params (OverlappedComponent :type "PrimitiveComponent Object Reference") (OtherActor :type "Actor Object Reference") (OtherComp :type "PrimitiveComponent Object Reference") (OtherBodyIndex :type Integer) (bFromSweep :type Boolean) (SweepResult :type "HitResult Structure (by ref)"))
  (if (== OtherActor (`self.PlayerChar`))
    (`self.StartToMoveChar`)))

(event `StartToMoveChar`
  (if (`self.CanBePickedUp`) :!label _label
    (if (`self.CheckInventoryForPickingUp` true)
      (set `self.VectorInterp` (`self.K2_GetActorLocation`)) ; Set loot initial location
      (`self.SetActorTickEnabled` true) ; Enable Tick to move loot to\nmain char
      (`KismetSystemLibrary.K2_SetTimerDelegate` (delegate `CustomEvent_0`) 0.5) ; If Loot doesn't taken after certain time, \nthen trigger an event to be taken
    )
    (else
      (`KismetSystemLibrary.Delay` 0.2) ; Wait for boolean to be true
      (goto _label))))

(event `CustomEvent_0`
  (if (not (`self.IsPickedUp`))
    (`self.BeforePickedUp`)))

(event `self.ReceiveTick`
  (params (DeltaSeconds :type "Float (single-precision)"))
  (if (`self.CheckInventoryForPickingUp` false)
    (set `self.PlayerLoc` (`self.K2_GetActorLocation` (`self.PlayerChar`)))
    (set `self.VectorInterp` (`KismetMathLibrary.VInterpTo` (`self.VectorInterp`) (`self.PlayerLoc`) (`GameplayStatics.GetWorldDeltaSeconds`) 7.0))
    (`self.K2_SetActorLocation` (`self.VectorInterp`))
    (if (<= (`KismetMathLibrary.VSize` (- (`self.VectorInterp`) (`self.PlayerLoc`))) 50.0)
      (`self.BeforePickedUp`))))

(event `PickedUp`
  ;[1 1 1] For child BPs
  (`/Engine/EditorBlueprintResources/StandardMacros.IsValid` (`self.PlayerChar`)
    (:`Is Valid`
      (bind _output_get (set `self.PlayerLootComp` (`self.GetComponentByClass` (`self.PlayerChar`) "/Game/Defender/Blueprints/Components/LootComp.LootComp_C"))) ; Get Player Loot Comp
      (`/Engine/EditorBlueprintResources/StandardMacros.IsValid` _output_get
        (:`Is Valid`
          (`/Game/Defender/Blueprints/Components/LootComp.AcquireLoot` (`self.PlayerLootComp`) (`GameplayStatics.GetObjectClass` self)) ; Loot is acquired
          (`self.K2_DestroyActor`))))))

(fn `ActivateProjectileMovement`
  (if (not (`self.IsProjectileMovementActivated`))
    (set `self.IsProjectileMovementActivated` true)
    (`ActorComponent.Activate` (`self.ProjectileMovement`) false) ; Activate Projectile Movement \nto throwing the loot
  ))

(fn `BeforePickedUp`
  (`self.SetActorTickEnabled` false) ; Disable Tick because of \nLoot is picked up
  (`GameplayStatics.PlaySoundAtLocation` (`self.PickedUpSound`) (`self.K2_GetActorLocation`) (struct) 1.0 1.0 0.0 "/Game/Defender/Demo/Audio/Attenuations/ATT_Loot.ATT_Loot" "/Game/Defender/Demo/Audio/Concurrencies/Con_Loot.Con_Loot" null null) ; Play sound when loot is picked up
  (`self.PickedUp`) ; PickedUp Event for child actors
  (set `self.IsPickedUp` true))

(fn `CheckInventoryForPickingUp`
  (params (ShowMessage :type Boolean))
  (returns (Return :type Boolean))
  (locals (LootClass :type "/Game/Defender/Blueprints/Loots/BP_LootParent Class Reference") (InventoryComp :type "/Game/Defender/Blueprints/Components/InventoryComp Object Reference") (Message :type Text) (Result :type Boolean :default false) (InShowMessage :type Boolean :default true))
  (bind _inventorycomp (`local.InventoryComp`))
  (bind _inventorycomp_2 (`local.InventoryComp`))
  (set `local.InShowMessage` ShowMessage)
  (set `local.LootClass` (`GameplayStatics.GetObjectClass` self))
  (if (== (`local.LootClass`) "/Game/Defender/Blueprints/Loots/OtherLoots/BP_LootMedkit.BP_LootMedkit_C")
    (set `local.InventoryComp` (`/Game/Defender/Blueprints/Characters/BP_MainCharParent.InventoryComp` (`self.GetMainChar`)))
    (bind _output_get (set `local.Result` (< (`/Game/Defender/Blueprints/Components/InventoryComp.MedkitCount` _inventorycomp) (`/Game/Defender/Blueprints/Components/InventoryComp.MaxMedkitCount` _inventorycomp))))
    (if (not _output_get)
      (`/Game/Defender/Blueprints/BP_MyPlayerController.ShowInfoMessage` (`self.GetPC`) "Can't carry any more medkits" (`local.InShowMessage`)))
    (return (`local.Result`))
    (elif (== (`local.LootClass`) "/Game/Defender/Blueprints/Loots/OtherLoots/BP_LootGrenade.BP_LootGrenade_C")
      (set `local.InventoryComp` (`/Game/Defender/Blueprints/Characters/BP_MainCharParent.InventoryComp` (`self.GetMainChar`)))
      (bind _output_get_2 (set `local.Result` (< (`/Game/Defender/Blueprints/Components/InventoryComp.GrenadeCount` _inventorycomp_2) (`/Game/Defender/Blueprints/Components/InventoryComp.MaxGrenadeCount` _inventorycomp_2))))
      (if (not _output_get_2)
        (`/Game/Defender/Blueprints/BP_MyPlayerController.ShowInfoMessage` (`self.GetPC`) "Can't carry any more grenades" (`local.InShowMessage`)))
      (return (`local.Result`))
      (else
        (return true)))))

(fn `GetMainChar`
  (returns (MainChar :type "/Game/Defender/Blueprints/Characters/BP_MainCharParent Object Reference"))
  (`/Engine/EditorBlueprintResources/StandardMacros.IsValid` (`self.MainChar`)
    (:`Is Valid`
      _)
    (:`Is Not Valid`
      (bind _asbp_main_char_parent (cast `/Game/Defender/Blueprints/Characters/BP_MainCharParent` (`GameplayStatics.GetPlayerCharacter` 0)))
      (set `self.MainChar` _asbp_main_char_parent)))
  (return (`self.MainChar`)))

(fn `GetPC`
  (returns (Pc :type "/Game/Defender/Blueprints/BP_MyPlayerController Object Reference"))
  (`/Engine/EditorBlueprintResources/StandardMacros.IsValid` (`self.Pc`) ; Valid Checking Of Player Controller. If it is valid, then we don't need to cast
    (:`Is Valid`
      _)
    (:`Is Not Valid`
      (bind _asbp_my_player_controller (cast `/Game/Defender/Blueprints/BP_MyPlayerController` (`GameplayStatics.GetPlayerController` 0))
        (:`then`
          (set `self.Pc` _asbp_my_player_controller))
        (:`CastFailed`
          (return null)))))
  (return (`self.Pc`)))

(fn `UserConstructionScript`)