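; Inventory component that tracks the owner's gold, medkits, grenades, weapons and per-projectile ammo.
; Change functions update counts (bounded for gold, medkits and grenades), broadcast dispatchers for UI and show messages through a cached player controller.
; Weapons and ammo live in class-keyed maps; NextWeapon cycles the weapons through WeaponComp when not reloading or firing.
; BeginPlay retries every 0.2 seconds until WeaponComp exists, then caches the owner's skeletal mesh.
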(event `self.ReceiveBeginPlay`
  (bind _output_get (set `self.WeaponComp` (`Actor.GetComponentByClass` (`self.GetOwner`) "/Game/Defender/Blueprints/Components/WeaponComp.WeaponComp_C")))
  (`/Engine/EditorBlueprintResources/StandardMacros.IsValid` _output_get :!label _label
    (:`Is Valid`
      (set `self.OwnerSkMesh` (`Actor.GetComponentByClass` (`self.GetOwner`) "/Script/Engine.SkeletalMeshComponent")))
    (:`Is Not Valid`
      (`KismetSystemLibrary.Delay` 0.2)
      (goto _label))))

(fn `AddUniqueWeaponWithRef`
  (params (WeaponClass :type "/Game/Defender/Blueprints/Weapons/BP_WeaponParent Class Reference") (WeaponObject :type "/Game/Defender/Blueprints/Weapons/BP_WeaponParent Object Reference"))
  (`BlueprintMapLibrary.Map_Add` (`self.WeaponRefs`) WeaponClass WeaponObject))

(fn `CanChangeWeapon`
  (returns (NewParam :type Boolean))
  (return (and (not (`/Game/Defender/Blueprints/Components/WeaponComp.isReloading` (`self.WeaponComp`))) (not (`/Game/Defender/Blueprints/Components/WeaponComp.isFiringPressed` (`self.WeaponComp`))) (> (`BlueprintMapLibrary.Map_Length` (`self.WeaponRefs`)) 1))))

(fn `ChangeGold`
  (params (ChangingGold :type Integer) (ShowMessage :type Boolean))
  (locals (InChangingGold :type Integer) (CalculatedGoldCount :type Integer :default 0) (InShowMessage :type Boolean))
  (set `local.InChangingGold` ChangingGold)
  (set `local.InShowMessage` ShowMessage)
  (set `local.CalculatedGoldCount` (+ (`self.GoldCount`) (`local.InChangingGold`)))
  (if (>= (`local.CalculatedGoldCount`) 0)
    (set `self.GoldCount` (`local.CalculatedGoldCount`))
    (`self.OnGoldChanged` (`local.InChangingGold`) (`local.CalculatedGoldCount`)) ; Broadcast Event Dispatcher \nfor updating UI etc.
    (`/Game/Defender/Blueprints/BP_MyPlayerController.ShowInfoMessage` (`self.GetPC`) (`|FormatText` "+{GoldCount} Gold" (`local.InChangingGold`)) (`local.InShowMessage`))
    (else
      (`/Game/Defender/Blueprints/BP_MyPlayerController.ShowInfoMessage` (`self.GetPC`) "Not enough gold!" true))))

(fn `ChangeGrenade`
  (params (ChangingGrenade :type Integer) (ShowMessage :type Boolean :default false))
  (locals (InChangingGrenade :type Integer) (NewGrenadeCount :type Integer :default 0) (InShowMessage :type Boolean))
  (bind _pc (`self.GetPC`))
  (set `local.InChangingGrenade` ChangingGrenade)
  (set `local.InShowMessage` ShowMessage)
  (set `local.NewGrenadeCount` (+ (`local.InChangingGrenade`) (`self.GrenadeCount`)))
  (if (>= (`local.NewGrenadeCount`) 0)
    (if (not (> (`local.NewGrenadeCount`) (`self.MaxGrenadeCount`)))
      (bind _output_get (set `self.GrenadeCount` (`local.NewGrenadeCount`)))
      (`self.OnGrenadeChanged` (`local.InChangingGrenade`) _output_get)
      (`/Engine/EditorBlueprintResources/StandardMacros.IsValid` _pc
        (:`Is Valid`
          (`/Game/Defender/Blueprints/BP_MyPlayerController.ShowInfoMessage` _pc (`|FormatText` "+{ChangingGrenade} Grenade" (`local.InChangingGrenade`)) (`local.InShowMessage`))))
      (else
        (`/Game/Defender/Blueprints/BP_MyPlayerController.ShowInfoMessage` (`self.GetPC`) "You can't carry more grenade" true)))
    (else
      (`/Game/Defender/Blueprints/BP_MyPlayerController.ShowInfoMessage` (`self.GetPC`) "Not enough grenade!" true))))

(fn `ChangeInvAmmoCount`
  (params (Projectile :type "/Game/Defender/Blueprints/Projectiles/BP_ProjectileParent Class Reference (by ref)") (ChangingAmmo :type "Integer (by ref)"))
  (locals (InProjectile :type "/Game/Defender/Blueprints/Projectiles/BP_ProjectileParent Class Reference") (InChangingAmmo :type Integer) (NewAmmoCount :type Integer :default 0))
  (set `local.InProjectile` Projectile)
  (set `local.InChangingAmmo` ChangingAmmo)
  (set `local.NewAmmoCount` (+ (`local.InChangingAmmo`) (`self.GetAmmoCount` (`local.InProjectile`))))
  (`self.SetInvAmmoCount` (`local.InProjectile`) (`local.NewAmmoCount`))
  (`self.OnInvAmmoChanged` (`local.InProjectile`) (`local.InChangingAmmo`) (`local.NewAmmoCount`)) ; Broadcast Event Dispatcher \nfor updating UI etc.
  (`/Game/Defender/Blueprints/BP_MyPlayerController.ShowInfoMessage` (`self.GetPC`) (`|FormatText` "+{ChangingAmmo} {ProjectileName} Ammo" (`local.InChangingAmmo`) (`.DisplayName` (defaults `Object` (`local.InProjectile`)))) true))

(fn `ChangeMedkit`
  (params (ChangingMedkit :type Integer) (ShowMessage :type Boolean))
  (locals (InChangingMedkit :type Integer) (InShowMessage :type Boolean))
  (set `local.InChangingMedkit` ChangingMedkit)
  (set `local.InShowMessage` ShowMessage)
  (bind _output_get (set `self.MedkitCount` (`KismetMathLibrary.Clamp` (+ ChangingMedkit (`self.MedkitCount`)) 0 (`self.MaxMedkitCount`))))
  (`self.OnMedkitChanged` (`local.InChangingMedkit`) _output_get) ; Broadcast Event Dispatcher \nfor updating UI etc.
  (`/Game/Defender/Blueprints/BP_MyPlayerController.ShowInfoMessage` (`self.GetPC`) (`|FormatText` "+{MedkitCount} Medkit" (`local.InChangingMedkit`)) (`local.InShowMessage`)))

(fn `GetAmmoCount`
  (params (ProjectileClass :type "/Game/Defender/Blueprints/Projectiles/BP_ProjectileParent Class Reference"))
  (returns (AmmoCount :type Integer))
  (locals (InProjectile :type "/Game/Defender/Blueprints/Projectiles/BP_ProjectileParent Class Reference") (InAmmoCount :type Integer))
  (bind (_value _returnvalue) (`BlueprintMapLibrary.Map_Find` (`self.InventoryAmmoCounts`) ProjectileClass))
  (if _returnvalue
    (return _value)
    (else
      (return 0))))

(fn `GetPC`
  (returns (Pc :type "/Game/Defender/Blueprints/BP_MyPlayerController Object Reference"))
  (`/Engine/EditorBlueprintResources/StandardMacros.IsValid` (`self.Pc`) ; Valid Checking Of Player Controller. If it is valid, then we don't need to cast
    (:`Is Valid`
      _)
    (:`Is Not Valid`
      (bind _asbp_my_player_controller (cast `/Game/Defender/Blueprints/BP_MyPlayerController` (`GameplayStatics.GetPlayerController` 0))
        (:`then`
          (set `self.Pc` _asbp_my_player_controller))
        (:`CastFailed`
          (return null)))))
  (return (`self.Pc`)))

(fn `GetWeaponObjectReference`
  (params (WeaponClass :type "/Game/Defender/Blueprints/Weapons/BP_WeaponParent Class Reference"))
  (returns (WeaponRef :type "/Game/Defender/Blueprints/Weapons/BP_WeaponParent Object Reference"))
  (bind (_value _returnvalue) (`BlueprintMapLibrary.Map_Find` (`self.WeaponRefs`) WeaponClass))
  (if _returnvalue
    (return _value)
    (else
      (return null))))

(fn `NextWeapon`
  (locals (ArrayIndex :type Integer :default 0) (WeaponsLength :type Integer :default 0) (NextIndex :type Integer :default 0) (WeaponKeys :type "Array of /Game/Defender/Blueprints/Weapons/BP_WeaponParent Class Reference"))
  (if (`self.CanChangeWeapon`)
    (`/Game/Defender/Blueprints/Components/WeaponComp.StopFiring` (`self.WeaponComp`))
    (bind _keys (`BlueprintMapLibrary.Map_Keys` (`self.WeaponRefs`)))
    (set `local.WeaponKeys` _keys)
    (set `local.ArrayIndex` (`KismetArrayLibrary.Array_Find` (`local.WeaponKeys`) (`GameplayStatics.GetObjectClass` (`self.EquippedWeapon`))))
    (set `local.NextIndex` (+ (`local.ArrayIndex`) 1))
    (if (>= (`local.NextIndex`) (`BlueprintMapLibrary.Map_Length` (`self.WeaponRefs`)))
      (set `local.NextIndex` 0))
    (`/Game/Defender/Blueprints/Components/WeaponComp.EquipWeapon` (`self.WeaponComp`) (`|GetArrayItem` (`local.WeaponKeys`) (`local.NextIndex`)) (`self.OwnerSkMesh`))))

(fn `SetInvAmmoCount`
  (params (Projectile :type "/Game/Defender/Blueprints/Projectiles/BP_ProjectileParent Class Reference") (AmmoCount :type Integer))
  (`BlueprintMapLibrary.Map_Add` (`self.InventoryAmmoCounts`) Projectile AmmoCount))