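; HpWidgetComp is a widget component that shows a health bar for its owning actor via a WB_Hp widget.
; On BeginPlay it passes the owner and its display name, visibility options and bar size into the widget.
; GetWidgetComp lazily casts the component's user widget to WB_Hp and caches the reference.
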(event `self.ReceiveBeginPlay`
  (`/Engine/EditorBlueprintResources/StandardMacros.IsValid` (`self.GetWidgetComp`)
    (:`Is Valid`
      (set `/Game/Defender/Blueprints/WidgetBP/WB_Hp.ParentActor` (`self.GetOwner`) (`self.GetWidgetComp`)) ; Transfer variable\nto WB_HPBar Widget
      (`/Game/Defender/Blueprints/WidgetBP/WB_Hp.Set Display Name` (`self.GetWidgetComp`) (`self.DisplayName`)) ; Transfer variable\nto WB_HPBar Widget
      (set `/Game/Defender/Blueprints/WidgetBP/WB_Hp.PreventShowIfHpFull` (`self.PreventShowIfHpFull`) (`self.GetWidgetComp`)) ; Transfer variable\nto WB_HPBar Widget
      (set `/Game/Defender/Blueprints/WidgetBP/WB_Hp.HideHpBar` (`self.HideHpBar`) (`self.GetWidgetComp`)) ; Transfer variable\nto WB_HPBar Widget
      (set `/Game/Defender/Blueprints/WidgetBP/WB_Hp.HPBarSize` (`self.HPBar Size`) (`self.GetWidgetComp`)) ; Transfer variable\nto WB_HPBar Widget
    )))

(fn `GetWidgetComp`
  (returns (Output_Get :type "/Game/Defender/Blueprints/WidgetBP/WB_Hp Object Reference"))
  (`/Engine/EditorBlueprintResources/StandardMacros.IsValid` (`self.WidgetComp`)
    (:`Is Valid`
      _)
    (:`Is Not Valid`
      (bind _aswb_hp (cast `/Game/Defender/Blueprints/WidgetBP/WB_Hp` (`self.GetUserWidgetObject`)))
      (set `self.WidgetComp` _aswb_hp)))
  (return (`self.WidgetComp`)))