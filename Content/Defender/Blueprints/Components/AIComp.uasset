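; AIComp is an actor component that starts and configures enemy AI for its owning pawn.
; On BeginPlay it gets the owner's BP_EnemyController, runs the assigned behavior tree, then seeds the blackboard with the player character as TargetActor and the configured AIBehaviourType.
; SetAIState writes a state enum to the blackboard's State key.
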(event `self.ReceiveBeginPlay`
  (bind _returnvalue (`AIBlueprintHelperLibrary.GetBlackboard` (`self.EnemyController`)))
  (set `self.Owner` (`self.GetOwner`))
  (bind _asbp_enemy_controller (cast `/Game/Defender/Blueprints/AI/AIControllers/BP_EnemyController` (`AIBlueprintHelperLibrary.GetAIController` (`self.Owner`))))
  (bind _output_get (set `self.EnemyController` _asbp_enemy_controller))
  (bind _returnvalue_2 (`AIController.RunBehaviorTree` _output_get (`self.BehaviourTree`)))
  (if _returnvalue_2
    (`BlackboardComponent.SetValueAsObject` _returnvalue "TargetActor" (`GameplayStatics.GetPlayerCharacter` 0)) ; Set Blackboard key TargetActor as Player Character
    (`BlackboardComponent.SetValueAsEnum` _returnvalue "AIBehaviourType" (`self.AIBehaviourType`))))

(fn `SetAIState`
  (params (State :type "/Game/Defender/StructsAndEnums/AiStateEnum Enum" :default "NewEnumerator4"))
  (`BlackboardComponent.SetValueAsEnum` (`AIBlueprintHelperLibrary.GetBlackboard` (`self.EnemyController`)) "State" State))