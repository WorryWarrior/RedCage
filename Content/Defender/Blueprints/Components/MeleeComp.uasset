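; MeleeComp is a component that deals melee damage for its owning actor, using the owner's skeletal mesh.
; While tracing is enabled, each Tick runs a multi box trace between two mesh sockets against two object types.
; Each actor hit takes random ranged point damage once per strike, with a scaled hit direction and the owner's AI controller as instigator.
; StrikeEnd clears the affected-actor list so targets can be hit again.
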(event `self.ReceiveBeginPlay`
  (bind _output_get (set `self.OwnerActor` (`self.GetOwner`)))
  (set `self.OwnerSK` (`Actor.GetComponentByClass` _output_get "/Script/Engine.SkeletalMeshComponent")))

(event `self.ReceiveTick`
  (params (DeltaSeconds :type "Float (single-precision)"))
  (if (`self.MeleeTraceEnabled`)
    (bind (_outhits _returnvalue) (`KismetSystemLibrary.BoxTraceMultiForObjects` (`self.GetSocketLocation` (`self.CollisionStartSocketName`)) (`self.GetSocketLocation` (`self.CollisionEndSocketName`)) (`self.MeleeTraceHalfSize`) (`SceneComponent.GetSocketRotation` (`self.OwnerSK`) (`self.CollisionStartSocketName`)) (`|MakeArray` "ObjectTypeQuery8" "ObjectTypeQuery9" :!type "EObjectTypeQuery Enum")))
    (if _returnvalue
      (for _array_element _outhits
        (set `self.Hit` _array_element)
        (set `self.Hit Actor` (`.HitActor` (`GameplayStatics.BreakHitResult` (`self.Hit`))))
        (if (not (`KismetArrayLibrary.Array_Contains` (`self.AffectedActors`) (`self.Hit Actor`)))
          (`KismetArrayLibrary.Array_Add` (`self.AffectedActors`) (`self.Hit Actor`))
          (`GameplayStatics.ApplyPointDamage` (`self.Hit Actor`) (`self.DetermineDamage`) (* (`self.CalculateHitDirection`) (`self.ImpulseMultiplier`)) (`self.Hit`) (`AIBlueprintHelperLibrary.GetAIController` (`self.OwnerActor`)) (`self.OwnerActor`) "/Script/Engine.DamageType"))))))

(fn `CalculateHitDirection`
  (returns (ReturnValue :type "Vector Structure"))
  (bind (_bblockinghit _binitialoverlap _time _distance _location _impactpoint _normal _impactnormal _physmat _hitactor _hitcomponent _hitbonename) (`GameplayStatics.BreakHitResult` (`self.Hit`)))
  (return (`KismetMathLibrary.Normal` (- (`SceneComponent.GetSocketLocation` _hitcomponent _hitbonename) (- (`self.GetSocketLocation` (`self.CollisionStartSocketName`)) (`self.GetSocketLocation` (`self.CollisionEndSocketName`)))) 0.01)))

(fn `DetermineDamage`
  (returns (ReturnValue :type "Float (double-precision)"))
  (return (`KismetMathLibrary.Conv_IntToDouble` (`KismetMathLibrary.RandomIntegerInRange` (`self.MeleeDamageMin`) (`self.MeleeDamageMax`)))))

(fn `GetSocketLocation`
  (params (SocketName :type Name))
  (returns (ReturnValue :type "Vector Structure"))
  (return (`SceneComponent.GetSocketLocation` (`self.OwnerSK`) SocketName)))

(fn `StrikeEnd`
  (`KismetArrayLibrary.Array_Clear` (`self.AffectedActors`)))