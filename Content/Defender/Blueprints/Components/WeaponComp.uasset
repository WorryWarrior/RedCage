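; Actor component that handles a character's weapon equipping, firing, reload start and save-game restore.
; It spawns or re-shows weapons held by InventoryComp, attaches them to a mesh socket and broadcasts weapon and ammo changes.
; Held fire loops on the weapon's cooldown, gated by health, reload and throw state; reloading notifies AnimComp.
; On owner death, the weapon detaches, falls with physics, dissolves and is destroyed.
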(event `self.ReceiveBeginPlay`
  (set `self.OwnerActor` (`self.GetOwner`)) ; Get parent actor which owned this comp
  (`/Engine/EditorBlueprintResources/StandardMacros.IsValid` (`self.OwnerActor`)
    (:`Is Valid`
      (set `self.OwnerSkMesh` (`Actor.GetComponentByClass` (`self.OwnerActor`) "/Script/Engine.SkeletalMeshComponent"))
      (bind _output_get (set `self.HealthComp` (`Actor.GetComponentByClass` (`self.OwnerActor`) "/Game/Defender/Blueprints/Components/HealthComp.HealthComp_C")))
      (add `/Game/Defender/Blueprints/Components/HealthComp.OnDeath` _output_get (delegate `OnDeath_Event_0`)) ; Bind event when owner death
      (set `self.AnimComp` (`Actor.GetComponentByClass` (`self.OwnerActor`) "/Game/Defender/Blueprints/Components/AnimComp.AnimComp_C")) ; Set Anim Comp for animating owner
      (set `self.InventoryComp` (`Actor.GetComponentByClass` (`self.OwnerActor`) "/Game/Defender/Blueprints/Components/InventoryComp.InventoryComp_C"))
      (set `self.ThrowComp` (`Actor.GetComponentByClass` (`self.OwnerActor`) "/Game/Defender/Blueprints/Components/ThrowComp.ThrowComp_C"))
      (`KismetSystemLibrary.Delay` 0.2)
      (`self.EquipWeapon` (`self.FirstEquipWeaponClass`) (`self.OwnerSkMesh`)) ; Spawn weapon and attach to weapon socket
    )))

(event `OnDeath_Event_0`
  (params (BoneName :type Name) (ShotFromDirection :type "Vector Structure") (HitComponent :type "PrimitiveComponent Object Reference"))
  (bind _equippedweapon (`self.GetInvEquippedWeapon`))
  (bind _equippedweapon_2 (`self.GetInvEquippedWeapon`))
  (bind _mesh (`/Game/Defender/Blueprints/Weapons/BP_WeaponParent.Mesh` (`self.Equipped Weapon`)))
  (bind _dissolvecomp (`/Game/Defender/Blueprints/Weapons/BP_WeaponParent.DissolveComp` _equippedweapon_2))
  (`/Engine/EditorBlueprintResources/StandardMacros.IsValid` HitComponent
    (:`Is Valid`
      (`KismetSystemLibrary.Delay` 0.1)
      (`/Engine/EditorBlueprintResources/StandardMacros.IsValid` _equippedweapon
        (:`Is Valid`
          (`Actor.K2_DetachFromActor` _equippedweapon "KeepWorld" "KeepWorld" "KeepWorld") ; Detach equipped weapon
          (`self.Activate` (`/Game/Defender/Blueprints/Weapons/BP_WeaponParent.RotatingMovement` (`self.GetInvEquippedWeapon`)) false) ; Activa rotation when weapon is falling
          (bind _output_get (set `self.Equipped Weapon` (`self.GetInvEquippedWeapon`)))
          (`PrimitiveComponent.SetCollisionEnabled` _mesh "PhysicsOnly") ; For allowing equipped weapon to falling\nthe ground
          (`PrimitiveComponent.SetSimulatePhysics` _mesh true)
          (`PrimitiveComponent.AddImpulse` _mesh (* ShotFromDirection 500.0) "None" false) ; Add small impulse according to \nShotFromDirection
          (`PrimitiveComponent.SetRenderCustomDepth` (`/Game/Defender/Blueprints/Weapons/BP_WeaponParent.Mesh` (`self.GetInvEquippedWeapon`)) false) ; Remove outline
          (`KismetSystemLibrary.Delay` (`self.WeaponDissolveStartDelay`))
          (`/Game/Defender/Blueprints/Components/DissolveComp.Execute` _dissolvecomp (`/Game/Defender/Blueprints/Weapons/BP_WeaponParent.Mesh` _equippedweapon_2)) ; Weapon Dissolve onDeath
          (add `/Game/Defender/Blueprints/Components/DissolveComp.DissolveCompleted` _dissolvecomp (delegate `DissolveCompleted`)) ; Call event when dissolve is completed
        )))))

(event `DissolveCompleted`
  (`Actor.K2_DestroyActor` (`self.GetInvEquippedWeapon`)))

(event `StartFiring`
  (params (TargetLocation :type "Vector Structure"))
  (set `self.TargetLocation` TargetLocation)
  (set `self.isFiringPressed` true)
  (if (`self.CanStartFiring`) :!label _label
    (set `self.isInFiringCooldown` true)
    (`/Engine/EditorBlueprintResources/StandardMacros.IsValid` (`self.GetInvEquippedWeapon`)
      (:`Is Valid`
        (`/Game/Defender/Blueprints/Weapons/BP_WeaponParent.Fire` (`self.GetInvEquippedWeapon`) (`self.TargetLocation`)) ; Fire equipped weapon
        (`KismetSystemLibrary.RetriggerableDelay` (`self.Get Equipped Weapon Cooldown`)) ; Delay of equipped weapon rate of fire
        (set `self.isInFiringCooldown` false)
        (goto _label))
      (:`Is Not Valid`
        (`self.StopFiring`)))))

(event `StopFiring`
  (bind _equippedweapon (`self.GetInvEquippedWeapon`))
  (set `self.isFiringPressed` false)
  (set `self.isInFiringCooldown` false)
  (`self.DeactiveMuzzle`)
  (`/Engine/EditorBlueprintResources/StandardMacros.IsValid` _equippedweapon
    (:`Is Valid`
      (`/Game/Defender/Blueprints/Weapons/BP_WeaponParent.DeactivateLazerSight` _equippedweapon))))

(event `AttemptToReload`
  (`/Engine/EditorBlueprintResources/StandardMacros.IsValid` (`self.GetInvEquippedWeapon`)
    (:`Is Valid`
      (if (`self.CanReloadEquippedWeapon`)
        (set `self.isReloading` true)
        (`self.StopFiring`)
        (`GameplayStatics.PlaySoundAtLocation` "/Game/Defender/Demo/Audio/Weapons/AssaultRifle/SCue_AR_Reload.SCue_AR_Reload" (`Actor.K2_GetActorLocation` (`self.OwnerActor`)) (struct) 1.0 1.0 0.0 "/Game/Defender/Demo/Audio/Attenuations/ATT_Reload.ATT_Reload" null null null)
        (`self.OnReloadStart`)
        (`/Game/Defender/Blueprints/Components/AnimComp.OnAnimStateChanged` (`self.AnimComp`) "NewEnumerator1")))))

(event `LoadEquippedWeapon`
  (params (SaveGame :type "/Game/Defender/Blueprints/SaveGames/SG_MainCharInventory Object Reference"))
  (set `self.SG` SaveGame)
  (set `self.FirstEquipWeaponClass` (`/Game/Defender/Blueprints/SaveGames/SG_MainCharInventory.EquippedWeaponClass` (`self.SG`)))
  (`/Engine/EditorBlueprintResources/StandardMacros.IsValid` (`self.InventoryComp`) :!label _label_2
    (:`Is Valid`
      (`/Engine/EditorBlueprintResources/StandardMacros.IsValid` (`self.GetInvEquippedWeapon`) :!label _label_3
        (:`Is Valid`
          (`self.EquipWeapon` (`/Game/Defender/Blueprints/SaveGames/SG_MainCharInventory.EquippedWeaponClass` (`self.SG`)) (`self.OwnerSkMesh`))
          (`/Game/Defender/Blueprints/Weapons/BP_WeaponParent.OnWeaponAmmoChanged` (`self.GetInvEquippedWeapon`) (`/Game/Defender/Blueprints/Weapons/BP_WeaponParent.GetMagazineAmmo` (`self.GetInvEquippedWeapon`)) (`/Game/Defender/Blueprints/Weapons/BP_WeaponParent.GetInvAmmoCount` (`self.GetInvEquippedWeapon`)))
          (set `self.isFiringPressed` false)
          (set `self.isInFiringCooldown` false))
        (:`Is Not Valid`
          (`KismetSystemLibrary.Delay` 0.2)
          (goto _label_3))))
    (:`Is Not Valid`
      (`KismetSystemLibrary.Delay` 0.2)
      (goto _label_2))))

(fn `CanReloadEquippedWeapon`
  (returns (CanReload :type Boolean))
  (bind _equippedweapon (`self.GetInvEquippedWeapon`))
  (bind _equippedweapon_2 (`self.GetInvEquippedWeapon`))
  (return (and (and (< (`/Game/Defender/Blueprints/Weapons/BP_WeaponParent.GetMagazineAmmo` _equippedweapon_2) (`/Game/Defender/Blueprints/Weapons/BP_WeaponParent.MagazineSize` _equippedweapon_2)) (!= (`/Game/Defender/Blueprints/Weapons/BP_WeaponParent.GetInvAmmoCount` _equippedweapon_2) 0)) (not (`self.isReloading`)) (not (`/Game/Defender/Blueprints/Components/ThrowComp.IsInThrowCooldown` (`self.ThrowComp`))) (`KismetMathLibrary.BooleanNAND` (<= (`/Game/Defender/Blueprints/Weapons/BP_WeaponParent.GetMagazineAmmo` _equippedweapon) 0) (<= (`/Game/Defender/Blueprints/Weapons/BP_WeaponParent.GetInvAmmoCount` _equippedweapon) 0)))))

(fn `CanStartFiring`
  (returns (ReturnValue :type Boolean))
  (return (and (`self.isFiringPressed`) (not (`self.isReloading`)) (`/Game/Defender/Blueprints/Components/HealthComp.isAlive` (`self.HealthComp`)) (not (`self.isInFiringCooldown`)) (not (`/Game/Defender/Blueprints/Components/ThrowComp.IsInThrowCooldown` (`self.ThrowComp`))))))

(fn `DeactiveMuzzle`
  (locals (EquippedWeapon :type "/Game/Defender/Blueprints/Weapons/BP_WeaponParent Object Reference"))
  (bind _output_get (set `local.EquippedWeapon` (`self.GetInvEquippedWeapon`)))
  (`/Engine/EditorBlueprintResources/StandardMacros.IsValid` _output_get
    (:`Is Valid`
      (`self.Deactivate` (`/Game/Defender/Blueprints/Weapons/BP_WeaponParent.MuzzleParticle` (`local.EquippedWeapon`))))))

(fn `EquipWeapon`
  (params (Class :type "/Game/Defender/Blueprints/Weapons/BP_WeaponParent Class Reference") (Mesh :type "SkeletalMeshComponent Object Reference"))
  (returns (EquippedWeapon :type "/Game/Defender/Blueprints/Weapons/BP_WeaponParent Object Reference"))
  (locals (Weapons :type "Array of  Structure") (InMesh :type "SkeletalMeshComponent Object Reference") (WeaponClass :type "/Game/Defender/Blueprints/Weapons/BP_WeaponParent Class Reference") (WeaponsMap :type "Map of /Game/Defender/Blueprints/Weapons/BP_WeaponParent Class Reference to /Game/Defender/Blueprints/Weapons/BP_WeaponParent Object Reference") (EquippedInvWeapon :type "/Game/Defender/Blueprints/Weapons/BP_WeaponParent Object Reference") (WeaponRef :type "/Game/Defender/Blueprints/Weapons/BP_WeaponParent Object Reference"))
  (bind _equippedweapon (`self.GetInvEquippedWeapon`))
  (set `local.InMesh` Mesh)
  (bind _output_get (set `local.WeaponClass` Class))
  (if (`KismetSystemLibrary.IsValidClass` _output_get)
    (`self.HideAllWeapons`)
    (set `local.WeaponRef` (`/Game/Defender/Blueprints/Components/InventoryComp.GetWeaponObjectReference` (`self.InventoryComp`) (`local.WeaponClass`)))
    (`/Engine/EditorBlueprintResources/StandardMacros.IsValid` (`local.WeaponRef`)
      (:`Is Valid`
        (set `/Game/Defender/Blueprints/Components/InventoryComp.EquippedWeapon` (`local.WeaponRef`) (`self.InventoryComp`))
        (`SceneComponent.SetVisibility` (`/Game/Defender/Blueprints/Weapons/BP_WeaponParent.Mesh` (`local.WeaponRef`)) true false))
      (:`Is Not Valid`
        (bind _returnvalue (`|SpawnActorFromClass` (`local.WeaponClass`) (`KismetMathLibrary.MakeTransform` (0.0 0.0 0.0)) "AdjustIfPossibleButAlwaysSpawn" "SelectDefaultAtRuntime" (`self.GetOwner`) self (`self.IsWeaponsFlashlightVisible`) null)) ; Spawn weapon
        (set `/Game/Defender/Blueprints/Components/InventoryComp.EquippedWeapon` _returnvalue (`self.InventoryComp`))))
    (`/Game/Defender/Blueprints/Components/InventoryComp.AddUniqueWeaponWithRef` (`self.InventoryComp`) (`local.WeaponClass`) (`self.GetInvEquippedWeapon`))
    (`Actor.K2_AttachToComponent` (`self.GetInvEquippedWeapon`) (`local.InMesh`) (`self.Socket Name`) "KeepRelative" "KeepRelative" "KeepRelative" true) ; Attach the spawned weapon to weapon socket
    (`self.OnEquippedWeaponChange` (`local.WeaponClass`) (`self.GetInvEquippedWeapon`) (`local.InMesh`)) ; Inform listeners\neg. Inventory
    (`/Game/Defender/Blueprints/Weapons/BP_WeaponParent.OnWeaponAmmoChanged` _equippedweapon (`/Game/Defender/Blueprints/Weapons/BP_WeaponParent.GetMagazineAmmo` _equippedweapon) (`/Game/Defender/Blueprints/Weapons/BP_WeaponParent.GetInvAmmoCount` _equippedweapon)) ; Call Equipped weapon Ammo Change\nEvent dispatcher
    (`GameplayStatics.PlaySoundAtLocation` "/Game/Defender/Demo/Audio/Weapons/AssaultRifle/SCue_AR_Equip.SCue_AR_Equip" (`Actor.K2_GetActorLocation` (`self.OwnerActor`)) (struct) 1.0 1.0 0.0 null null null null)
    (return (`self.GetInvEquippedWeapon`))
    (else
      (`KismetSystemLibrary.PrintString` "First weapon class is not defined in Weapon Comp!" true true (struct :`R` 1.0 :`B` 0.027883 :`A` 1.0) 100.0))))

(fn `Get Equipped Weapon Cooldown`
  (returns (ReturnValue :type "Float (double-precision)"))
  (return (`/Game/Defender/Blueprints/Weapons/BP_WeaponParent.GetCooldownDelay` (`self.GetInvEquippedWeapon`))))

(fn `GetEquippedWeapon`
  (returns (EquippedWeapon :type "/Game/Defender/Blueprints/Weapons/BP_WeaponParent Object Reference"))
  (return (`/Game/Defender/Blueprints/Components/InventoryComp.EquippedWeapon` (`self.InventoryComp`))))

(fn `GetInvEquippedWeapon`
  (returns (EquippedWeapon :type "/Game/Defender/Blueprints/Weapons/BP_WeaponParent Object Reference"))
  (return (`/Game/Defender/Blueprints/Components/InventoryComp.EquippedWeapon` (`self.InventoryComp`))))

(fn `HideAllWeapons`
  (locals (WeaponRef :type "/Game/Defender/Blueprints/Weapons/BP_WeaponParent Object Reference"))
  (bind _values (`BlueprintMapLibrary.Map_Values` (`/Game/Defender/Blueprints/Components/InventoryComp.WeaponRefs` (`self.InventoryComp`))))
  (for _array_element _values
    (set `local.WeaponRef` _array_element)
    (`/Engine/EditorBlueprintResources/StandardMacros.IsValid` (`local.WeaponRef`)
      (:`Is Valid`
        (`SceneComponent.SetVisibility` (`/Game/Defender/Blueprints/Weapons/BP_WeaponParent.Mesh` (`local.WeaponRef`)) false false)))))

(fn `Reset`
  (set `self.isFiringPressed` false)
  (set `self.isInFiringCooldown` false)
  (set `self.isReloading` false))