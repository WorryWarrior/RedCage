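; Health component that tracks its owning actor's health, death state and medkit healing.
; It binds to the owner's point and radial damage events, caching bone, hit component and shot direction before applying damage.
; ChangeHealth clamps the value and broadcasts OnHealthChanged, plus OnDeath with the cached hit data at zero health.
; UseMedkit spends a medkit from InventoryComp to heal with sound, particles and a short cooldown.
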(event `self.ReceiveBeginPlay`
  (bind _output_get (set `self.OwnerActor` (`self.GetOwner`))) ; Get Owner Actor
  (`/Engine/EditorBlueprintResources/StandardMacros.IsValid` _output_get
    (:`Is Valid`
      (set `self.OwnerSK` (`Actor.GetComponentByClass` (`self.OwnerActor`) "/Script/Engine.SkeletalMeshComponent"))
      (set `self.InventoryComp` (`Actor.GetComponentByClass` (`self.OwnerActor`) "/Game/Defender/Blueprints/Components/InventoryComp.InventoryComp_C"))
      (add `Actor.OnTakePointDamage` (`self.OwnerActor`) (`|CreateDelegate` :!event `TakePointDamageEvent`)) ; Call event when actor take point damage\neg. take a bullet
      (add `Actor.OnTakeRadialDamage` (`self.OwnerActor`) (`|CreateDelegate` :!event `RadialDamageEvent`)) ; Call event when actor take radial damage\neg. damage from grenades
      (`self.SetHealthPercent`))))

(event `UseMedkit`
  (if (> (`/Game/Defender/Blueprints/Components/InventoryComp.MedkitCount` (`self.InventoryComp`)) 0)
    (if (and (not (`self.IsInUsingMedkitCooldown`)) (< (`self.HealthPercent`) 1.0))
      (set `self.IsInUsingMedkitCooldown` true)
      (`/Game/Defender/Blueprints/Components/InventoryComp.ChangeMedkit` (`self.InventoryComp`) -1 false)
      (`self.ChangeHealth` (`self.MedkitHealthBenefit`))
      (`GameplayStatics.PlaySound2D` "/Game/Defender/Demo/Audio/Other/SCue_Heal.SCue_Heal" 1.0 1.0 0.0 null null)
      (`GameplayStatics.SpawnEmitterAttached` (`self.MedkitParticle`) (`self.OwnerSK`) "None" (`KismetMathLibrary.MakeVector` 0.0 0.0 (`self.MedkitParticleOffsetZ`)) (struct) (1.0 1.0 1.0) "KeepRelativeOffset" true "AutoRelease")
      (`KismetSystemLibrary.Delay` 1.0)
      (set `self.IsInUsingMedkitCooldown` false))
    (else
      (`/Game/Defender/Blueprints/BP_MyPlayerController.ShowInfoMessage` (`self.GetPC`) "Not enough medkit" true))))

(event `TakePointDamageEvent`
  (params (DamagedActor :type "Actor Object Reference") (Damage :type "Float (single-precision)") (InstigatedBy :type "Controller Object Reference") (HitLocation :type "Vector Structure") (FHitComponent :type "PrimitiveComponent Object Reference") (BoneName :type Name) (ShotFromDirection :type "Vector Structure") (DamageType :type "DamageType Object Reference") (DamageCauser :type "Actor Object Reference"))
  (if (`self.isAlive`)
    (set `self.Shot from Direction` ShotFromDirection)
    (set `self.Bone Name` BoneName)
    (set `self.Hit Component` FHitComponent)
    (`self.ChangeHealth` (* Damage -1.0))))

(event `RadialDamageEvent`
  (params (DamagedActor :type "Actor Object Reference") (Damage :type "Float (single-precision)") (DamageType :type "DamageType Object Reference") (Origin :type "Vector Structure") (HitInfo :type "HitResult Structure") (InstigatedBy :type "Controller Object Reference") (DamageCauser :type "Actor Object Reference"))
  (bind (_bblockinghit _binitialoverlap _time _distance _location _impactpoint _normal _impactnormal _physmat _hitactor _hitcomponent _hitbonename) (`GameplayStatics.BreakHitResult` HitInfo))
  (if (`self.isAlive`)
    (set `self.Damage Causer` DamageCauser)
    (set `self.Shot from Direction` (* (`KismetMathLibrary.Normal` (- (`Actor.K2_GetActorLocation` (`self.OwnerActor`)) Origin)) 2.0))
    (set `self.Bone Name` _hitbonename)
    (set `self.Hit Component` _hitcomponent)
    (`self.ChangeHealth` (* (`KismetMathLibrary.Conv_IntToDouble` (`KismetMathLibrary.Round` Damage)) -1.0))))

(fn `ChangeHealth`
  (params (ChangingHealth :type "Float (double-precision)"))
  (locals (InChangingHealth :type "Float (double-precision)"))
  (set `local.InChangingHealth` ChangingHealth)
  (if (and (not (== (`local.InChangingHealth`) 0.0)) (`self.isAlive`))
    (set `self.Health` (`KismetMathLibrary.FClamp` (+ (`self.Health`) (`local.InChangingHealth`)) 0.0 (`self.MaxHealth`)))
    (set `self.HealthPercent` (/ (`self.Health`) (`self.MaxHealth`)))
    (`self.OnHealthChanged` (`local.InChangingHealth`) (`self.Health`) (`self.MaxHealth`) (`self.HealthPercent`)) ; Call onHealthChange dispatcher to all listener BPs
    (if (<= (`self.Health`) 0.0)
      (set `self.isAlive` false)
      (`self.OnDeath` (`self.Bone Name`) (`self.Shot from Direction`) (`self.Hit Component`)) ; Call onDeath dispatcher to all listener BPs\nif health is below zero
    )))

(fn `ChangeMaxHealth`
  (params (MaxHealth :type "Float (double-precision)"))
  (set `self.MaxHealth` (`KismetMathLibrary.FClamp` MaxHealth (`self.Health`) MaxHealth)))

(fn `GetPC`
  (returns (Pc :type "/Game/Defender/Blueprints/BP_MyPlayerController Object Reference"))
  (`/Engine/EditorBlueprintResources/StandardMacros.IsValid` (`self.Pc`) ; Valid Checking Of Player Controller. If it is valid, then we don't need to cast
    (:`Is Valid`
      _)
    (:`Is Not Valid`
      (bind _asbp_my_player_controller (cast `/Game/Defender/Blueprints/BP_MyPlayerController` (`GameplayStatics.GetPlayerController` 0))
        (:`then`
          (set `self.Pc` _asbp_my_player_controller))
        (:`CastFailed`
          (return null)))))
  (return (`self.Pc`)))

(fn `SetHealthPercent`
  (set `self.HealthPercent` (/ (`self.Health`) (`self.MaxHealth`))))