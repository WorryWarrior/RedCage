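; Actor component that drops loot when its owner dies and applies picked-up loot to its owner.
; On HealthComp death, it spawns fixed loot classes plus a random count from a weighted map, using staggered delays and randomized yaw.
; Weighted picks roll per entry, falling back to a uniform choice.
; AcquireLoot switches on loot type to update InventoryComp or equip through WeaponComp, with random ammo matched to the player's weapons.
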(event `self.ReceiveBeginPlay`
  (`/Engine/EditorBlueprintResources/StandardMacros.IsValid` (`self.GetOwner`)
    (:`Is Valid`
      (set `self.OwnerSkMesh` (`Actor.GetComponentByClass` (`self.GetOwner`) "/Script/Engine.SkeletalMeshComponent"))
      (set `self.InventoryComp` (`Actor.GetComponentByClass` (`self.GetOwner`) "/Game/Defender/Blueprints/Components/InventoryComp.InventoryComp_C"))
      (set `self.WeaponComp` (`Actor.GetComponentByClass` (`self.GetOwner`) "/Game/Defender/Blueprints/Components/WeaponComp.WeaponComp_C"))
      (`self.BindOnDeath`))))

(event `BindOnDeath`
  (bind _output_get (set `self.HealthComp` (`Actor.GetComponentByClass` (`self.GetOwner`) "/Game/Defender/Blueprints/Components/HealthComp.HealthComp_C"))) ; Get Health Comp for \ndetermining owner is death
  (`/Engine/EditorBlueprintResources/StandardMacros.IsValid` _output_get
    (:`Is Valid`
      (add `/Game/Defender/Blueprints/Components/HealthComp.OnDeath` (`self.HealthComp`) (delegate `OnDeath`)) ; Call event when owner is death
    )))

(event `OnDeath`
  (params (BoneName :type Name) (ShotFromDirection :type "Vector Structure") (HitComponent :type "PrimitiveComponent Object Reference"))
  (`self.SpawnLoot` ShotFromDirection))

(event `SpawnLoot`
  (params (Direction :type "Vector Structure (by ref)"))
  (set `self.Direction` Direction)
  (set `self.LootLocation` (`self.GetLootLocation`))
  (`self.SpawnSpecificLoots` (`self.Direction`)) ; Spawn specific loot classes
  (`self.SpawnRandomLoots` (`self.Direction`)) ; Spawn randomized loots
)

(event `SpawnSpecificLoots`
  (params (Direction :type "Vector Structure (by ref)"))
  (set `self.SpecificLootDirection` Direction)
  (bind _output_get (set `self.SpecificLootsLength` (`KismetArrayLibrary.Array_Length` (`self.SpecificLoots`))))
  (if (> _output_get 0)
    (set `self.SpecificLootClass` (`|GetArrayItem` (`self.SpecificLoots`) (`self.SpecificLootIndex`)) :!label _label)
    (if (`KismetSystemLibrary.IsValidClass` (`self.SpecificLootClass`))
      (`|SpawnActorFromClass` (`self.SpecificLootClass`) (`KismetMathLibrary.MakeTransform` (`self.LootLocation`) (`self.GetLootRotation` (`self.SpecificLootDirection`))) "AdjustIfPossibleButAlwaysSpawn" "SelectDefaultAtRuntime" null false null) ; Spawn given Loot Class
      (`self.PlayLootSpawnSound`)
      (`KismetSystemLibrary.Delay` 0.2))
    (`/Engine/EditorBlueprintResources/StandardMacros.IncrementInt` (`self.SpecificLootIndex`) ; Next Index of Array
      (:`  `
        (if (< (`self.SpecificLootIndex`) (`self.SpecificLootsLength`))
          (goto _label))))))

(event `SpawnRandomLoots`
  (params (Direction :type "Vector Structure"))
  (set `self.RandomLootDirection` Direction)
  (if (> (`BlueprintMapLibrary.Map_Length` (`self.RandomLootsMap`)) 0)
    (`/Engine/EditorBlueprintResources/StandardMacros.Do N` (`KismetMathLibrary.RandomIntegerInRange` (`self.RandomLootMin`) (`self.RandomLootMax`)) :!label _label_2
      (:`Exit`
        (bind _output_get (set `self.DeterminedLoot` (`self.DetermineLootClass`)))
        (if (`KismetSystemLibrary.IsValidClass` _output_get)
          (`|SpawnActorFromClass` (`self.DeterminedLoot`) (`KismetMathLibrary.MakeTransform` (`self.LootLocation`) (`self.GetLootRotation` (`self.RandomLootDirection`))) "AlwaysSpawn" "SelectDefaultAtRuntime" null false null) ; Spawn random Loot Classes
          (`self.PlayLootSpawnSound`)
          (`KismetSystemLibrary.Delay` 0.2) ; Delay between loot spawns
          (goto _label_2)
          (else
            (goto _label_2)))))))

(fn `AcquireLoot`
  (params (Loot :type "/Game/Defender/Blueprints/Loots/BP_LootParent Class Reference"))
  (locals (InLoot :type "/Game/Defender/Blueprints/Loots/BP_LootParent Class Reference") (WeaponClass :type "/Game/Defender/Blueprints/Weapons/BP_WeaponParent Class Reference"))
  (set `local.InLoot` Loot)
  (`/Engine/EditorBlueprintResources/StandardMacros.IsValid` (`self.GetPC`)
    (:`Is Valid`
      (switch `/Game/Defender/StructsAndEnums/LootTypeEnum` (defaults `Object` (`local.InLoot`)) ; Switch according to\nLootType
        (:`NewEnumerator0`
          (`/Game/Defender/Blueprints/Components/InventoryComp.ChangeGold` (`self.InventoryComp`) 100 true))
        (:`NewEnumerator1`
          (`/Game/Defender/Blueprints/Components/InventoryComp.ChangeMedkit` (`self.InventoryComp`) 1 true))
        (:`NewEnumerator2`
          (`self.AddRandomAmmo`))
        (:`NewEnumerator5`
          (`self.AddSpecificAmmo` (`local.InLoot`)))
        (:`NewEnumerator4`
          (`/Game/Defender/Blueprints/Components/InventoryComp.ChangeGrenade` (`self.InventoryComp`) 1 true))
        (:`NewEnumerator3`
          (bind _asbp_loot_weapon_parent (castclass `/Game/Defender/Blueprints/Loots/BP_LootWeaponParent` (`local.InLoot`)))
          (set `local.WeaponClass` (defaults `Object` _asbp_loot_weapon_parent))
          (`/Game/Defender/Blueprints/Components/WeaponComp.EquipWeapon` (`self.WeaponComp`) (`local.WeaponClass`) (`self.OwnerSkMesh`))
          (`/Game/Defender/Blueprints/BP_MyPlayerController.ShowInfoMessage` (`self.GetPC`) (`|FormatText` "You acquired a {WP}" (defaults `Object` (`local.WeaponClass`))) true))))))

(fn `AddRandomAmmo`
  (locals (SelectedProjectile :type "/Game/Defender/Blueprints/Projectiles/BP_ProjectileParent Class Reference") (SelectedAmmoCount :type Integer :default 0) (RandomAmmoIndex :type Integer :default 0) (Keys :type "Array of /Game/Defender/Blueprints/Weapons/BP_WeaponParent Class Reference") (SelectedWeaponClass :type "/Game/Defender/Blueprints/Weapons/BP_WeaponParent Class Reference"))
  (bind _keys (`BlueprintMapLibrary.Map_Keys` (`/Game/Defender/Blueprints/Components/InventoryComp.WeaponRefs` (`/Game/Defender/Blueprints/Characters/BP_MainCharParent.InventoryComp` (`self.GetMainChar`)))))
  (set `local.Keys` _keys)
  (bind _output_get (set `local.SelectedWeaponClass` (`|GetArrayItem` (`local.Keys`) (`.OutIndex` (`KismetArrayLibrary.Array_Random` (`local.Keys`))))))
  (if (`KismetSystemLibrary.IsValidClass` _output_get)
    (set `local.SelectedProjectile` (defaults `Object` (`local.SelectedWeaponClass`))) ; Select a random projectile\naccording to inventory weapons
    (set `local.SelectedAmmoCount` (`KismetMathLibrary.RandomIntegerInRange` 10 50))
    (`/Game/Defender/Blueprints/Components/InventoryComp.ChangeInvAmmoCount` (`self.InventoryComp`) (`local.SelectedProjectile`) (`local.SelectedAmmoCount`))
    (else
      (`KismetSystemLibrary.PrintString` "InventoryComp Weapons Variable is not set properly!" true true (struct :`G` 0.66 :`B` 1.0 :`A` 1.0) 100.0))))

(fn `AddSpecificAmmo`
  (params (Loot :type "/Game/Defender/Blueprints/Loots/BP_LootParent Class Reference"))
  (locals (SelectedAmmoCount :type Integer))
  (bind _asbp_loot_specific_ammo_parent (castclass `/Game/Defender/Blueprints/Loots/BP_LootSpecificAmmoParent` Loot))
  (set `local.SelectedAmmoCount` (`KismetMathLibrary.RandomIntegerInRange` 5 15))
  (`/Game/Defender/Blueprints/Components/InventoryComp.ChangeInvAmmoCount` (`self.InventoryComp`) (defaults `Object` _asbp_loot_specific_ammo_parent) (`local.SelectedAmmoCount`)))

(fn `DetermineLootClass`
  (returns (DeterminedLoot :type "/Game/Defender/Blueprints/Loots/BP_LootParent Class Reference"))
  (locals (TotalWeight :type "Float (double-precision)") (LootsArray :type "Array of /Game/Defender/Blueprints/Loots/BP_LootParent Class Reference") (Loot :type "/Game/Defender/Blueprints/Loots/BP_LootParent Class Reference") (RandomLootWeights :type "Array of Float (double-precision)"))
  (bind _values (`BlueprintMapLibrary.Map_Values` (`self.RandomLootsMap`)))
  (set `local.RandomLootWeights` _values)
  (for _array_element (`local.RandomLootWeights`)
    (set `local.TotalWeight` (+ (`local.TotalWeight`) _array_element)))
  (bind _keys (`BlueprintMapLibrary.Map_Keys` (`self.RandomLootsMap`)))
  (for _array_element_2 _keys
    (set `local.Loot` _array_element_2)
    (`KismetArrayLibrary.Array_Add` (`local.LootsArray`) (`local.Loot`))
    (if (> (`BlueprintMapLibrary.Map_Find` (`self.RandomLootsMap`) (`local.Loot`)) (`KismetMathLibrary.RandomFloatInRange` 0.0 (`local.TotalWeight`)))
      (return (`local.Loot`))))
  (return (`KismetArrayLibrary.Array_Random` (`local.LootsArray`))))

(fn `GetLootLocation`
  (returns (ReturnValue :type "Vector Structure"))
  (bind (_returnvalue_x _returnvalue_y _returnvalue_z) (`KismetMathLibrary.BreakVector` (`Actor.K2_GetActorLocation` (`self.GetOwner`))))
  (return (`KismetMathLibrary.MakeVector` _returnvalue_x _returnvalue_y (+ _returnvalue_z (`self.LootOffsetZ`)))))

(fn `GetLootRotation`
  (params (Y :type "Vector Structure (by ref)"))
  (returns (ReturnValue :type "Rotator Structure"))
  (bind (_returnvalue_roll _returnvalue_pitch) (`KismetMathLibrary.BreakRotator` (`KismetMathLibrary.MakeRotFromY` Y)))
  (return (`KismetMathLibrary.MakeRotator` 0.0 0.0 (+ (* _returnvalue_pitch -1.0) (`KismetMathLibrary.RandomFloatInRange` -90.0 90.0)))))

(fn `GetMainChar`
  (returns (MainChar :type "/Game/Defender/Blueprints/Characters/BP_MainCharParent Object Reference"))
  (`/Engine/EditorBlueprintResources/StandardMacros.IsValid` (`self.MainChar`)
    (:`Is Valid`
      _)
    (:`Is Not Valid`
      (bind _asbp_main_char_parent (cast `/Game/Defender/Blueprints/Characters/BP_MainCharParent` (`GameplayStatics.GetPlayerCharacter` 0)))
      (set `self.MainChar` _asbp_main_char_parent)))
  (return (`self.MainChar`)))

(fn `GetPC`
  (returns (Pc :type "/Game/Defender/Blueprints/BP_MyPlayerController Object Reference"))
  (`/Engine/EditorBlueprintResources/StandardMacros.IsValid` (`self.Pc`) ; Valid Checking Of Player Controller. If it is valid, then we don't need to cast
    (:`Is Valid`
      _)
    (:`Is Not Valid`
      (bind _asbp_my_player_controller (cast `/Game/Defender/Blueprints/BP_MyPlayerController` (`GameplayStatics.GetPlayerController` 0))
        (:`then`
          (set `self.Pc` _asbp_my_player_controller))
        (:`CastFailed`
          (return null)))))
  (return (`self.Pc`)))

(fn `PlayLootSpawnSound`
  (`GameplayStatics.PlaySoundAtLocation` "/Game/Defender/Demo/Audio/Pickups/SCue_Hammer_Swing_Cue.SCue_Hammer_Swing_Cue" (`Actor.K2_GetActorLocation` (`self.GetOwner`)) (struct) 1.0 1.0 0.0 null null (`self.GetOwner`) null))