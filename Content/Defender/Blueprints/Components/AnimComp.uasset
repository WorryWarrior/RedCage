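; AnimComp is a component that plays the owner's reload and grenade toss montages and turns their notifies into gameplay calls.
; It caches the skeletal mesh and the throw, weapon and inventory components, then plays a montage section on each matching anim state change.
; Notifies complete the reload, spawn the grenade or end the throw.
; Interrupted montages clear the reloading flag or end the throw.
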(event `self.ReceiveBeginPlay`
  (set `self.OwnerActor` (`self.GetOwner`))
  (set `self.OwnerSk` (`Actor.GetComponentByClass` (`self.OwnerActor`) "/Script/Engine.SkeletalMeshComponent"))
  (set `self.ThrowComp` (`Actor.GetComponentByClass` (`self.OwnerActor`) "/Game/Defender/Blueprints/Components/ThrowComp.ThrowComp_C"))
  (set `self.WeaponComp` (`Actor.GetComponentByClass` (`self.OwnerActor`) "/Game/Defender/Blueprints/Components/WeaponComp.WeaponComp_C"))
  (set `self.InventoryComp` (`Actor.GetComponentByClass` (`self.OwnerActor`) "/Game/Defender/Blueprints/Components/InventoryComp.InventoryComp_C"))
  (add `self.OnAnimStateChanged` (`|CreateDelegate` :!event `AnimStateChanged`)))

(event `AnimStateChanged` :!signature `self.OnAnimStateChanged`
  (params (AnimState :type "/Game/Defender/StructsAndEnums/AnimState Enum" :default "NewEnumerator0"))
  (bind _output_get (set `self.Anim State` AnimState))
  (switch `/Game/Defender/StructsAndEnums/AnimState` _output_get
    (:`NewEnumerator1`
      (`|PlayMontage` (`self.OwnerSk`) "/Game/Defender/Demo/Animations/Soldier/AM_Mannequin.AM_Mannequin" 1.0 0.0 "Reload"
        (:`OnInterrupted`
          (`self.ReloadInterrupted`))))
    (:`NewEnumerator2`
      (`|PlayMontage` (`self.OwnerSk`) "/Game/Defender/Demo/Animations/Soldier/AM_Mannequin.AM_Mannequin" 1.0 0.0 "TossGrenade"
        (:`OnInterrupted`
          (`self.TossGrenadeInterrupted`))))))

(event `Notify`
  (params (NotifyName :type Name))
  (bind _inventorycomp (`self.InventoryComp`))
  (switch `name` NotifyName
    (:`Default`
      (`KismetSystemLibrary.PrintString` "There is an issue in notifies (AnimComp)"))
    (:`ReloadCompleted`
      (`/Engine/EditorBlueprintResources/StandardMacros.IsValid` _inventorycomp
        (:`Is Valid`
          (`/Game/Defender/Blueprints/Weapons/BP_WeaponParent.Reload Completed Actions` (`/Game/Defender/Blueprints/Components/InventoryComp.EquippedWeapon` _inventorycomp))
          (set `/Game/Defender/Blueprints/Components/WeaponComp.isReloading` false (`self.WeaponComp`))
          (`/Game/Defender/Blueprints/Components/WeaponComp.OnReloadCompleted` (`self.WeaponComp`)))))
    (:`ThrowGrenade`
      (`/Game/Defender/Blueprints/Components/ThrowComp.SpawnGrenade` (`self.ThrowComp`)))
    (:`ThrowEnd`
      (`/Game/Defender/Blueprints/Components/ThrowComp.ThrowEnd` (`self.ThrowComp`)))))

(fn `ReloadInterrupted`
  (set `/Game/Defender/Blueprints/Components/WeaponComp.isReloading` false (`self.WeaponComp`)))

(fn `TossGrenadeInterrupted`
  (`/Game/Defender/Blueprints/Components/ThrowComp.ThrowEnd` (`self.ThrowComp`)))