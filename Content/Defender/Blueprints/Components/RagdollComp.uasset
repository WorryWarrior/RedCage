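; Actor component that ragdolls a character on death, driven by an Execute event receiving the capsule, mesh and hit details.
; It switches the mesh to physics-only simulation and pushes the hit bone along the shot direction with a randomized impulse.
; The capsule loses gravity and takes an after-death collision profile.
; For owners other than the first player, it teleports to world origin after a short delay, avoiding collision issues.
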(event `Execute`
  (params (CapsuleComponent :type "CapsuleComponent Object Reference") (Mesh :type "SkeletalMeshComponent Object Reference") (InHitComp :type "PrimitiveComponent Object Reference") (InBoneName :type Name) (InShotFromDirection :type "Vector Structure"))
  (set `self.CapsuleComponent` CapsuleComponent)
  (set `self.Mesh` Mesh)
  (set `self.InHitComp` InHitComp)
  (set `self.InBoneName` InBoneName)
  (set `self.InShotFromDirection` InShotFromDirection)
  (`PrimitiveComponent.SetCollisionProfileName` (`self.Mesh`) "CustomRagdoll" true)
  (`PrimitiveComponent.SetCollisionEnabled` (`self.Mesh`) "PhysicsOnly") ; Enable Physics Only Collision
  (`PrimitiveComponent.SetSimulatePhysics` (`self.Mesh`) true) ; Enable physics sim
  (`PrimitiveComponent.AddImpulse` (`self.Mesh`) (* (`self.InShotFromDirection`) (`KismetMathLibrary.RandomIntegerInRange` 35000 40000)) (`self.InBoneName`) false) ; Add impulse to mesh with shot from direction and \nadd impulse to mesh according to its physic asset
  (`PrimitiveComponent.SetEnableGravity` (`self.CapsuleComponent`) false)
  (`PrimitiveComponent.SetCollisionProfileName` (`self.CapsuleComponent`) "CapsuleAfterDeath" true)
  (if (!= (`self.GetOwner`) (`GameplayStatics.GetPlayerCharacter` 0))
    (`KismetSystemLibrary.Delay` 0.2)
    (`SceneComponent.K2_SetWorldLocation` (`self.CapsuleComponent`) (0.0 0.0 0.0) false true) ; Fix: Change capsule location for preventing collision issues
  ))