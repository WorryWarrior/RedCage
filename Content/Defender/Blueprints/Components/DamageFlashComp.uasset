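; Actor component that briefly flashes the owner's mesh material when it takes point or radial damage.
; On BeginPlay, if enabled, it creates colored dynamic materials for all static and skeletal mesh slots, stored in parallel component and material arrays.
; Each damage handler flashes the hit component's first stored material for a set duration behind a DoOnce gate.
; Radial damage clears a hardcoded "DamageSwitch" parameter instead of the configurable name.
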(event `self.ReceiveBeginPlay`
  (if (`self.IsEnabled`)
    (`self.CreateSMDynamicMats`)
    (`self.CreateSKDynamicMats`)
    (add `Actor.OnTakePointDamage` (`self.GetOwner`) (delegate `OnTakePointDamage_Event_0`))
    (add `Actor.OnTakeRadialDamage` (`self.GetOwner`) (delegate `OnTakeRadialDamage_Event_0`))))

(event `OnTakeRadialDamage_Event_0`
  (params (DamagedActor :type "Actor Object Reference") (Damage :type "Float (single-precision)") (DamageType :type "DamageType Object Reference") (Origin :type "Vector Structure") (HitInfo :type "HitResult Structure (by ref)") (InstigatedBy :type "Controller Object Reference") (DamageCauser :type "Actor Object Reference"))
  (set `self.RadialHitInfo` HitInfo)
  (`/Engine/EditorBlueprintResources/StandardMacros.DoOnce` false :!label _label
    (:`Completed`
      (set `self.DynamicMat` (`|GetArrayItem` (`self.DynamicMats`) (`KismetArrayLibrary.Array_Find` (`self.PrimitiveComps`) (`.HitComponent` (`GameplayStatics.BreakHitResult` (`self.RadialHitInfo`))))))
      (bind _dynamicmat (`self.DynamicMat`)
        (:`then`
          (`MaterialInstanceDynamic.SetScalarParameterValue` _dynamicmat (`self.MatParameterName`) 1.0)
          (`KismetSystemLibrary.Delay` (`self.FlashDuration`))
          (bind _dynamicmat_2 (`self.DynamicMat`)
            (:`then`
              (`MaterialInstanceDynamic.SetScalarParameterValue` _dynamicmat_2 "DamageSwitch" 0.0)
              (goto _label :!via `Reset`))
            (:`else`)))
        (:`else`)))))

(event `OnTakePointDamage_Event_0`
  (params (DamagedActor :type "Actor Object Reference") (Damage :type "Float (single-precision)") (InstigatedBy :type "Controller Object Reference") (HitLocation :type "Vector Structure") (FHitComponent :type "PrimitiveComponent Object Reference") (BoneName :type Name) (ShotFromDirection :type "Vector Structure") (DamageType :type "DamageType Object Reference") (DamageCauser :type "Actor Object Reference"))
  (set `self.HitComp` FHitComponent)
  (`/Engine/EditorBlueprintResources/StandardMacros.DoOnce` false :!label _label_2
    (:`Completed`
      (set `self.DynamicMat` (`|GetArrayItem` (`self.DynamicMats`) (`KismetArrayLibrary.Array_Find` (`self.PrimitiveComps`) (`self.HitComp`))))
      (bind _dynamicmat (`self.DynamicMat`)
        (:`then`
          (`MaterialInstanceDynamic.SetScalarParameterValue` _dynamicmat (`self.MatParameterName`) 1.0)
          (`KismetSystemLibrary.Delay` (`self.FlashDuration`))
          (bind _dynamicmat_2 (`self.DynamicMat`)
            (:`then`
              (`MaterialInstanceDynamic.SetScalarParameterValue` _dynamicmat_2 (`self.MatParameterName`) 0.0)
              (goto _label_2 :!via `Reset`))
            (:`else`)))
        (:`else`)))))

(fn `CreateSKDynamicMats`
  (locals (SKComps :type "Array of SkeletalMeshComponent Object Reference") (SKComp :type "SkeletalMeshComponent Object Reference") (SKTotalMatCount :type Integer :default 0) (InDynamicMat :type "MaterialInstanceDynamic Object Reference") (MaterialIndex :type Integer))
  (set `local.SKComps` (`Actor.K2_GetComponentsByClass` (`self.GetOwner`) "/Script/Engine.SkeletalMeshComponent"))
  (for _array_element (`local.SKComps`)
    (set `local.SKComp` _array_element)
    (bind _output_get (set `local.SKTotalMatCount` (`PrimitiveComponent.GetNumMaterials` (`local.SKComp`))))
    (for _index (range _output_get)
      (bind _output_get_2 (set `local.MaterialIndex` _index))
      (bind _returnvalue (`PrimitiveComponent.CreateDynamicMaterialInstance` (`local.SKComp`) _output_get_2 (`PrimitiveComponent.GetMaterial` (`local.SKComp`) (`local.MaterialIndex`)) "None"))
      (set `local.InDynamicMat` _returnvalue)
      (`KismetArrayLibrary.Array_Add` (`self.PrimitiveComps`) (`local.SKComp`))
      (`KismetArrayLibrary.Array_Add` (`self.DynamicMats`) (`local.InDynamicMat`))
      (`MaterialInstanceDynamic.SetVectorParameterValue` (`local.InDynamicMat`) "FlashColor" (`self.FlashColor`)))))

(fn `CreateSMDynamicMats`
  (locals (SMComps :type "Array of StaticMeshComponent Object Reference") (SMComp :type "StaticMeshComponent Object Reference") (MaterialIndex :type Integer) (InDynamicMat :type "MaterialInstanceDynamic Object Reference"))
  (bind _output_get (set `local.SMComps` (`Actor.K2_GetComponentsByClass` (`self.GetOwner`) "/Script/Engine.StaticMeshComponent")))
  (for _array_element _output_get
    (bind _output_get_2 (set `local.SMComp` _array_element))
    (bind _output_get_3 (set `self.SMTotalMatCount` (`PrimitiveComponent.GetNumMaterials` _output_get_2)))
    (for _index (range _output_get_3)
      (bind _output_get_4 (set `local.MaterialIndex` _index))
      (bind _returnvalue (`PrimitiveComponent.CreateDynamicMaterialInstance` (`local.SMComp`) (`local.MaterialIndex`) (`PrimitiveComponent.GetMaterial` (`local.SMComp`) _output_get_4) "None"))
      (set `local.InDynamicMat` _returnvalue)
      (`KismetArrayLibrary.Array_Add` (`self.PrimitiveComps`) (`local.SMComp`))
      (`KismetArrayLibrary.Array_Add` (`self.DynamicMats`) (`local.InDynamicMat`))
      (`MaterialInstanceDynamic.SetVectorParameterValue` (`local.InDynamicMat`) "FlashColor" (`self.FlashColor`)))))