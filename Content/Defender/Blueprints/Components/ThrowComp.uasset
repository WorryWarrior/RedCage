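; Actor component that handles grenade throwing for its owning actor, checking cooldown, health, reloading and grenade count before switching the animation state.
; Anim notifies call the spawn and end events: spawning launches BP_Grenade from the throw socket along a suggested arc toward the target, with randomly scaled impulse, and decrements inventory.
; Ending restores the animation state, clears the cooldown, resets the weapon and signals completion.
; Only a player owner sees the out-of-grenades message.
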(event `self.ReceiveBeginPlay`
  (set `self.OwnerActor` (`self.GetOwner`))
  (set `self.AnimComp` (`Actor.GetComponentByClass` (`self.OwnerActor`) "/Game/Defender/Blueprints/Components/AnimComp.AnimComp_C"))
  (set `self.HealthComp` (`Actor.GetComponentByClass` (`self.OwnerActor`) "/Game/Defender/Blueprints/Components/HealthComp.HealthComp_C"))
  (set `self.InventoryComp` (`Actor.GetComponentByClass` (`self.OwnerActor`) "/Game/Defender/Blueprints/Components/InventoryComp.InventoryComp_C"))
  (set `self.WeaponComp` (`Actor.GetComponentByClass` (`self.OwnerActor`) "/Game/Defender/Blueprints/Components/WeaponComp.WeaponComp_C")))

(event `ThrowStart`
  (params (Mesh :type "SceneComponent Object Reference"))
  (set `self.Mesh` Mesh)
  (if (`self.CanThrow`)
    (if (> (`/Game/Defender/Blueprints/Components/InventoryComp.GrenadeCount` (`self.InventoryComp`)) 0)
      (set `self.IsInThrowCooldown` true)
      (`/Game/Defender/Blueprints/Components/AnimComp.OnAnimStateChanged` (`self.AnimComp`) "NewEnumerator2") ; Animation state change to throwing
      (else
        (`/Game/Defender/Blueprints/BP_MyPlayerController.ShowInfoMessage` (`self.GetPC`) "Not enough grenade!" (`self.CheckIfOwnerIsPlayer`))
        (`self.ThrowEnd`)))))

(event `SpawnGrenade`
  (bind _owneractor (`self.OwnerActor`))
  (bind _throwsockettransform_location (`KismetMathLibrary.BreakTransform` (`self.ThrowSocketTransform`)))
  (bind _throwsockettransform_location_2 (`KismetMathLibrary.BreakTransform` (`self.ThrowSocketTransform`)))
  (if (`self.CanSpawnGrenade`)
    (set `self.ThrowSocketTransform` (`SceneComponent.GetSocketTransform` (`self.Mesh`) (`self.ThrowSocket`) "RTS_World"))
    (bind _outlaunchvelocity (`GameplayStatics.SuggestProjectileVelocity_CustomArc` _throwsockettransform_location_2 (`self.TargetLocation`) (`self.Override Gravity Z`) (`self.Arc Param`))) ; Calculate grenade velocity to arrive target location when tossed
    (`|SpawnActorFromClass` "/Game/Defender/Blueprints/Grenades/BP_Grenade.BP_Grenade_C" (`KismetMathLibrary.MakeTransform` _throwsockettransform_location (`self.ThrowRotation`)) "AlwaysSpawn" "OverrideRootScale" _owneractor (* _outlaunchvelocity (`KismetMathLibrary.RandomFloatInRange` 5.0 6.0)) (`Actor.Instigator` _owneractor)) ; Spawn grenade according to calculated velocity
    (`/Game/Defender/Blueprints/Components/InventoryComp.ChangeGrenade` (`self.InventoryComp`) -1 false)))

(event `ThrowEnd`
  (`/Game/Defender/Blueprints/Components/AnimComp.OnAnimStateChanged` (`self.AnimComp`) "NewEnumerator0")
  (`self.OnThrowEnded`)
  (set `self.IsInThrowCooldown` false)
  (`/Game/Defender/Blueprints/Components/WeaponComp.Reset` (`self.WeaponComp`)))

(fn `CanSpawnGrenade`
  (returns (ReturnValue :type Boolean))
  (return (`/Game/Defender/Blueprints/Components/HealthComp.isAlive` (`self.HealthComp`))))

(fn `CanThrow`
  (returns (ReturnValue :type Boolean))
  (return (and (not (`self.IsInThrowCooldown`)) (`/Game/Defender/Blueprints/Components/HealthComp.isAlive` (`self.HealthComp`)) (`KismetSystemLibrary.IsValid` (`self.InventoryComp`)) (not (`/Game/Defender/Blueprints/Components/WeaponComp.isReloading` (`self.WeaponComp`))))))

(fn `CheckIfOwnerIsPlayer`
  (returns (IsPlayer :type Boolean))
  (return (== (`self.OwnerActor`) (`GameplayStatics.GetPlayerCharacter` 0))))

(fn `GetPC`
  (returns (Pc :type "/Game/Defender/Blueprints/BP_MyPlayerController Object Reference"))
  (`/Engine/EditorBlueprintResources/StandardMacros.IsValid` (`self.Pc`) ; Valid Checking Of Player Controller. If it is valid, then we don't need to cast
    (:`Is Valid`
      _)
    (:`Is Not Valid`
      (bind _asbp_my_player_controller (cast `/Game/Defender/Blueprints/BP_MyPlayerController` (`GameplayStatics.GetPlayerController` 0))
        (:`then`
          (set `self.Pc` _asbp_my_player_controller))
        (:`CastFailed`
          (return null)))))
  (return (`self.Pc`)))