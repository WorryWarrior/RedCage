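; PhysicMatComp is a helper component that chooses bullet impact feedback and damage scaling from the physical material hit.
; Four independent lookup functions switch on surface type to return a scaled particle, a decal, a damage multiplier or a sound cue.
; Flesh and metal get their own sounds, and vulnerable flesh such as the head takes a caller-supplied multiplier.
; Every visible decal branch returns the same bullet decal.
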(fn `GetBulletSound`
  (params (Target :type "PhysicalMaterial Object Reference"))
  (returns (Sound :type "SoundBase Object Reference"))
  (switch `EPhysicalSurface` (`PhysicalMaterial.SurfaceType` Target)
    (:`SurfaceType_Default`
      (return "/Game/Defender/Demo/Audio/Impacts/SCue_Impt_Bullet_Default.SCue_Impt_Bullet_Default"))))

(fn `GetDamageMultiplier`
  (params (PhysicMat :type "PhysicalMaterial Object Reference") (VulnarableDamageMultiplier :type "Float (double-precision)" :default 10.0))
  (returns (DamageMultiplier :type "Float (double-precision)"))
  (switch `EPhysicalSurface` (`PhysicalMaterial.SurfaceType` PhysicMat)
    (:`SurfaceType_Default`
      (return 1.0))))

(fn `GetDecal`
  (params (PhysicMat :type "PhysicalMaterial Object Reference"))
  (returns (DecalMat :type "MaterialInterface Object Reference"))
  (switch `EPhysicalSurface` (`PhysicalMaterial.SurfaceType` PhysicMat)
    (:`SurfaceType_Default`
      (return "/Game/Defender/Demo/Materials/M_BulletDecal.M_BulletDecal"))))

(fn `GetParticleEffect`
  (params (PhysicalMat :type "PhysicalMaterial Object Reference"))
  (returns (Particle :type "ParticleSystem Object Reference") (Scale :type "Vector Structure"))
  (switch `EPhysicalSurface` (`PhysicalMaterial.SurfaceType` PhysicalMat)
    (:`SurfaceType_Default`
      (return "/Game/Defender/Demo/Particles/P_Impact.P_Impact" (0.5 0.5 0.5)))))