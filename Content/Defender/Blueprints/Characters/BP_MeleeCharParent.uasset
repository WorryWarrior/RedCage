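; BP_MeleeCharParent is the parent Blueprint for AI-controlled melee characters, handling their death and save-data restore.
; On HealthComp death it disables claw overlaps, limits capsule collision to WorldStatic so the body stays on the floor, and stops AI movement and logic.
; Timed steps then remove the custom-depth outline, run DissolveComp on the mesh and destroy the actor when dissolved.
; LoadActor restores transform and health from a saved struct.
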(event `self.HealthComp.OnDeath`
  (params (BoneName :type Name) (ShotFromDirection :type "Vector Structure") (HitComponent :type "PrimitiveComponent Object Reference"))
  (bind _returnvalue (`AIBlueprintHelperLibrary.GetAIController` self))
  (`self.DisableClawCollisions`) ; Disable claws so they cannot damage\nwhen dead
  (`PrimitiveComponent.SetCollisionResponseToAllChannels` (`self.CapsuleComponent`) "ECR_Ignore")
  (`PrimitiveComponent.SetCollisionResponseToChannel` (`self.CapsuleComponent`) "ECC_WorldStatic" "ECR_Block") ; For standing in game world\nwe must capsule comp collide with floor
  (`Controller.StopMovement` _returnvalue)
  (`BrainComponent.StopLogic` (`AIController.BrainComponent` _returnvalue) "")
  (`KismetSystemLibrary.K2_SetTimer` null "RemoveOutline" 2.0) ; Timer for removing outline
  (`KismetSystemLibrary.Delay` 5.0)
  (`/Game/Defender/Blueprints/Components/DissolveComp.Execute` (`self.DissolveComp`) (`self.Mesh`))
  (add `/Game/Defender/Blueprints/Components/DissolveComp.DissolveCompleted` (`self.DissolveComp`) (delegate `DissolveCompleted_Event_0`)))

(event `DissolveCompleted_Event_0`
  (`self.K2_DestroyActor`))

(fn `DisableClawCollisions`
  (for _array_element (`self.GetComponentsByTag` "/Script/Engine.BoxComponent" "Claw")
    (set `PrimitiveComponent.bGenerateOverlapEvents` false _array_element)))

(fn `LoadActor`
  (params (MeleeCharStruct :type "/Game/Defender/Blueprints/SaveGames/SaveGameStructs/MeleeCharsStruct Structure"))
  (locals (InStruct :type "/Game/Defender/Blueprints/SaveGames/SaveGameStructs/MeleeCharsStruct Structure") (EquippedWeapon :type "/Game/Defender/Blueprints/Weapons/BP_WeaponParent Object Reference"))
  (bind ((`Health_13_1C2B531547491A35E801F9A9FD7C7C6C` _health) (`MaxHealth_12_8C00E5014A8BF03AC36787B28DE23C2E` _maxhealth)) (break `/Game/Defender/Blueprints/SaveGames/SaveGameStructs/MeleeCharsStruct` (`local.InStruct`)))
  (set `local.InStruct` MeleeCharStruct)
  (`self.K2_SetActorTransform` (`.Transform_14_E6D0EC384EA76DAE00B0498F7DBC69BD` (break `/Game/Defender/Blueprints/SaveGames/SaveGameStructs/MeleeCharsStruct` (`local.InStruct`))))
  (`self.SetHealthMaxHealth` _health _maxhealth))

(fn `RemoveOutline`
  (`PrimitiveComponent.SetRenderCustomDepth` (`self.Mesh`) false) ; Remove outline
)

(fn `SetHealthMaxHealth`
  (params (Health :type "Float (double-precision)") (MaxHealth :type "Float (double-precision)"))
  (locals (OldHealth :type "Float (double-precision)" :default 0.0) (NewHealth :type "Float (double-precision)") (NewMaxHealth :type "Float (double-precision)"))
  (set `local.NewHealth` Health)
  (set `local.NewMaxHealth` MaxHealth)
  (set `local.OldHealth` (`/Game/Defender/Blueprints/Components/HealthComp.Health` (`self.HealthComp`)))
  (`/Game/Defender/Blueprints/Components/HealthComp.ChangeHealth` (`self.HealthComp`) (- (`local.NewHealth`) (`local.OldHealth`)))
  (`/Game/Defender/Blueprints/Components/HealthComp.ChangeMaxHealth` (`self.HealthComp`) (`local.NewMaxHealth`)))

(fn `UserConstructionScript`)