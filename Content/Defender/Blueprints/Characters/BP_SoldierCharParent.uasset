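; Parent Blueprint for soldier characters, built on health, ragdoll, dissolve, inventory and weapon components.
; On death it ragdolls from the hit, plays a sound, clears the custom-depth outline on a timer, then dissolves after a randomized delay and destroys itself.
; LoadActor restores transform, health, inventory and equipped weapon from a struct.
; The construction script converts local waypoints to world space, and helpers cache the player controller and destroy the equipped weapon.
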(event `self.HealthComp.OnDeath`
  (params (BoneName :type Name) (ShotFromDirection :type "Vector Structure") (HitComponent :type "PrimitiveComponent Object Reference"))
  (`/Game/Defender/Blueprints/Components/RagdollComp.Execute` (`self.RagdollComp`) (`self.CapsuleComponent`) (`self.Mesh`) HitComponent BoneName ShotFromDirection) ; Execute Ragdoll because of death
  (`GameplayStatics.PlaySoundAtLocation` (`self.DeathSound`) (`self.K2_GetActorLocation`) (struct) 1.0 1.0 0.0 null null null null)
  (`KismetSystemLibrary.K2_SetTimer` null "RemoveOutline" 2.0) ; Timer for removing outline
  (`KismetSystemLibrary.Delay` (+ (`self.DissolveStartDelay`) (`KismetMathLibrary.RandomFloatInRange` 1.0 3.0)))
  (`/Game/Defender/Blueprints/Components/DissolveComp.Execute` (`self.DissolveComp`) (`self.Mesh`)) ; Execute Dissolve because of death
)

(event `self.DissolveComp.DissolveCompleted`
  (`self.K2_DestroyActor`) ; Destroy Actor when dissolve completed
)

(fn `DestroyEquippedWeapon`
  (bind _equippedweapon (`/Game/Defender/Blueprints/Components/InventoryComp.EquippedWeapon` (`self.InventoryComp`)))
  (`/Engine/EditorBlueprintResources/StandardMacros.IsValid` _equippedweapon
    (:`Is Valid`
      (`self.K2_DestroyActor` _equippedweapon))))

(fn `GetPC`
  (returns (Pc :type "/Game/Defender/Blueprints/BP_MyPlayerController Object Reference"))
  (`/Engine/EditorBlueprintResources/StandardMacros.IsValid` (`self.Pc`) ; Get player controller reference once, if it is valid
    (:`Is Valid`
      _)
    (:`Is Not Valid`
      (bind _asbp_my_player_controller (cast `/Game/Defender/Blueprints/BP_MyPlayerController` (`GameplayStatics.GetPlayerController` 0))
        (:`then`
          (set `self.Pc` _asbp_my_player_controller))
        (:`CastFailed`
          (return null)))))
  (return (`self.Pc`)))

(fn `LoadActor`
  (params (EnemiesStruct :type "/Game/Defender/Blueprints/SaveGames/SaveGameStructs/SoldiersStruct Structure"))
  (locals (Struct :type "/Game/Defender/Blueprints/SaveGames/SaveGameStructs/SoldiersStruct Structure") (EquippedWeapon :type "/Game/Defender/Blueprints/Weapons/BP_WeaponParent Object Reference"))
  (bind ((`Health_13_1C2B531547491A35E801F9A9FD7C7C6C` _health) (`MaxHealth_12_8C00E5014A8BF03AC36787B28DE23C2E` _maxhealth)) (break `/Game/Defender/Blueprints/SaveGames/SaveGameStructs/SoldiersStruct` (`local.Struct`)))
  (set `local.Struct` EnemiesStruct)
  (`self.K2_SetActorTransform` (`.Transform_14_E6D0EC384EA76DAE00B0498F7DBC69BD` (break `/Game/Defender/Blueprints/SaveGames/SaveGameStructs/SoldiersStruct` (`local.Struct`))))
  (`self.SetHealthMaxHealth` _health _maxhealth)
  (set `/Game/Defender/Blueprints/Components/InventoryComp.WeaponRefs` (`.Weapons_45_6F94F5614DFB936CED4AC3A8DD3C1AF0` (break `/Game/Defender/Blueprints/SaveGames/SaveGameStructs/SoldiersStruct` (`local.Struct`))) (`self.InventoryComp`))
  (set `/Game/Defender/Blueprints/Components/InventoryComp.InventoryAmmoCounts` (`.AmmoCounts_44_CFC7A608464B5FF02477E0ACCA9A51EB` (break `/Game/Defender/Blueprints/SaveGames/SaveGameStructs/SoldiersStruct` (`local.Struct`))) (`self.InventoryComp`))
  (set `/Game/Defender/Blueprints/Components/InventoryComp.MedkitCount` (`.MedkitCount_32_5E3D428B4A99AC587BD28D845842F450` (break `/Game/Defender/Blueprints/SaveGames/SaveGameStructs/SoldiersStruct` (`local.Struct`))) (`self.InventoryComp`))
  (set `/Game/Defender/Blueprints/Components/InventoryComp.GrenadeCount` (`.GrenadeCount_31_FC464FFB4B3F470A2A0D589747A291D8` (break `/Game/Defender/Blueprints/SaveGames/SaveGameStructs/SoldiersStruct` (`local.Struct`))) (`self.InventoryComp`))
  (bind _equippedweapon (`/Game/Defender/Blueprints/Components/WeaponComp.EquipWeapon` (`self.WeaponComp`) (`.EquippedWeaponClass_33_3048E1F9446F7E3D3C6F2582E03BC308` (break `/Game/Defender/Blueprints/SaveGames/SaveGameStructs/SoldiersStruct` (`local.Struct`))) (`self.Mesh`)))
  (set `local.EquippedWeapon` _equippedweapon)
  (`/Game/Defender/Blueprints/Weapons/BP_WeaponParent.SetMagazineAmmo` (`local.EquippedWeapon`) (`/Game/Defender/Blueprints/Weapons/BP_WeaponParent.GetMagazineAmmo` (`local.EquippedWeapon`))))

(fn `ProjectWaypointsToWorldLocs`
  (for _array_element (`self.Waypoints`)
    (`KismetArrayLibrary.Array_Add` (`self.WaypointsWorld`) (`KismetMathLibrary.TransformLocation` (`self.GetTransform`) _array_element))))

(fn `RemoveOutline`
  (`PrimitiveComponent.SetRenderCustomDepth` (`self.Mesh`) false) ; Remove outline
)

(fn `SetHealthMaxHealth`
  (params (Health :type "Float (double-precision)") (MaxHealth :type "Float (double-precision)"))
  (locals (OldHealth :type "Float (double-precision)" :default 0.0) (NewHealth :type "Float (double-precision)") (NewMaxHealth :type "Float (double-precision)"))
  (set `local.NewHealth` Health)
  (set `local.NewMaxHealth` MaxHealth)
  (set `local.OldHealth` (`/Game/Defender/Blueprints/Components/HealthComp.Health` (`self.HealthComp`)))
  (`/Game/Defender/Blueprints/Components/HealthComp.ChangeHealth` (`self.HealthComp`) (- (`local.NewHealth`) (`local.OldHealth`)))
  (`/Game/Defender/Blueprints/Components/HealthComp.ChangeMaxHealth` (`self.HealthComp`) (`local.NewMaxHealth`)))

(fn `UserConstructionScript`
  (`self.ProjectWaypointsToWorldLocs`))