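; Behavior tree task that moves a soldier pawn to the next waypoint in its patrol route.
; It reads the world-space waypoint array from BP_SoldierCharParent and runs AI MoveTo toward the entry at the Blackboard WaypointIndex.
; Whether the move succeeds or fails, it advances the index, wrapping to zero at the end, and finishes successfully.
; An empty waypoint list also finishes successfully without moving.
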(event `self.ReceiveExecuteAI`
  (params (OwnerController :type "AIController Object Reference") (ControlledPawn :type "Pawn Object Reference"))
  (set `self.Controlled Pawn` ControlledPawn)
  (bind _output_get (set `self.WaypointsWorld` (`/Game/Defender/Blueprints/Characters/BP_SoldierCharParent.WaypointsWorld` (cast `/Game/Defender/Blueprints/Characters/BP_SoldierCharParent` (`self.Controlled Pawn`) :!pure true))))
  (bind _output_get_2 (set `self.WaypointsLength` (`KismetArrayLibrary.Array_Length` _output_get)))
  (if (> _output_get_2 0)
    (bind _output_get_3 (set `self.Destination` (`|GetArrayItem` (`self.WaypointsWorld`) (`self.GetWaypointIndex`))))
    (`|AIMoveTo` (`self.Controlled Pawn`) _output_get_3 null 10.0 true
      (:`OnSuccess`
        _)
      (:`OnFail`
        _))
    (`self.SetWaypointIndex` (`KismetMathLibrary.SelectInt` 0 (+ (`self.GetWaypointIndex`) 1) (>= (+ (`self.GetWaypointIndex`) 1) (`self.WaypointsLength`))))
    (`self.FinishExecute` true)
    (else
      (`self.FinishExecute` true))))

(fn `GetWaypointIndex`
  (returns (ReturnValue :type Integer))
  (return (`BTFunctionLibrary.GetBlackboardValueAsInt` (`self.WaypointIndex`))))

(fn `SetWaypointIndex`
  (params (Value :type Integer))
  (`BTFunctionLibrary.SetBlackboardValueAsInt` (`self.WaypointIndex`) Value))