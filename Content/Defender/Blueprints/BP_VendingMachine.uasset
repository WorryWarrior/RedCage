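; BP_VendingMachine is an interactable vending machine that opens a vending screen after the player stands in its trigger box long enough.
; Box overlap plays a timeline that drives the progress widget's percent, retrying after a short delay until that widget is valid.
; Leaving stops the timeline and zeroes the bar.
; Completion hides the widget and calls ShowVendingWidget on the cached BP_MyPlayerController, passing itself.
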(event `self.ReceiveBeginPlay`
  (bind _aswb_vending_progress (cast `/Game/Defender/Blueprints/WidgetBP/WB_VendingProgress` (`WidgetComponent.GetUserWidgetObject` (`self.ProgressWidgetComp`))))
  (set `self.VendingProgressWb` _aswb_vending_progress))

(event `self.Box.OnComponentBeginOverlap`
  (params (OverlappedComponent :type "PrimitiveComponent Object Reference") (OtherActor :type "Actor Object Reference") (OtherComp :type "PrimitiveComponent Object Reference") (OtherBodyIndex :type Integer) (bFromSweep :type Boolean) (SweepResult :type "HitResult Structure (by ref)"))
  (if (== (`GameplayStatics.GetPlayerCharacter` 0) OtherActor)
    (`self.StartProgressTimer`)))

(event `self.Box.OnComponentEndOverlap`
  (params (OverlappedComponent :type "PrimitiveComponent Object Reference") (OtherActor :type "Actor Object Reference") (OtherComp :type "PrimitiveComponent Object Reference") (OtherBodyIndex :type Integer))
  (if (== (`GameplayStatics.GetPlayerCharacter` 0) OtherActor)
    (`self.LeavedBeforeOpen`)))

(event `StartProgressTimer`
  (`/Engine/EditorBlueprintResources/StandardMacros.IsValid` (`self.VendingProgressWb`) :!label _label
    (:`Is Valid`
      (`Widget.SetVisibility` (`self.VendingProgressWb`) "Visible")
      (bind (_direction _newtrack_0) (`Timeline|ProgressTimer` :!via `PlayFromStart` :!label _label_2)
        (:`Update`
          (`/Game/Defender/Blueprints/WidgetBP/WB_VendingProgress.ChangePercent` (`self.VendingProgressWb`) _newtrack_0))
        (:`Finished`
          (`KismetSystemLibrary.Delay` 0.2)
          (`Widget.SetVisibility` (`self.VendingProgressWb`) "Hidden")
          (`self.OpenVendingScreen`))))
    (:`Is Not Valid`
      (`KismetSystemLibrary.Delay` 0.2)
      (goto _label))))

(event `StopTimer`
  (goto _label_2 :!via `Stop`))

(event `LeavedBeforeOpen`
  (`TimelineComponent.Stop` (`self.ProgressTimer`))
  (`/Game/Defender/Blueprints/WidgetBP/WB_VendingProgress.ChangePercent` (`self.VendingProgressWb`) 0.0))

(event `OpenVendingScreen`
  (`/Game/Defender/Blueprints/BP_MyPlayerController.ShowVendingWidget` (`self.GetPC`) self))

(fn `GetPC`
  (returns (Pc :type "/Game/Defender/Blueprints/BP_MyPlayerController Object Reference"))
  (`/Engine/EditorBlueprintResources/StandardMacros.IsValid` (`self.Pc`) ; Valid Checking Of Player Controller. If it is valid, then we don't need to cast
    (:`Is Valid`
      _)
    (:`Is Not Valid`
      (bind _asbp_my_player_controller (cast `/Game/Defender/Blueprints/BP_MyPlayerController` (`GameplayStatics.GetPlayerController` 0))
        (:`then`
          (set `self.Pc` _asbp_my_player_controller))
        (:`CastFailed`
          (return null)))))
  (return (`self.Pc`)))

(fn `UserConstructionScript`)