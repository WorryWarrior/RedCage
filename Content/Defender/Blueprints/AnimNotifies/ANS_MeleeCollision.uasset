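; Anim notify state that marks the window in a melee animation during which hit tracing is active.
; A shared helper finds the MeleeComp on the mesh's owner and, if valid, sets its MeleeTraceEnabled flag.
; Notify begin turns the flag on; notify end turns it off and calls StrikeEnd on the returned component.
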(fn `Received_NotifyBegin`
  (params (MeshComp :type "SkeletalMeshComponent Object Reference") (Animation :type "AnimSequenceBase Object Reference") (TotalDuration :type "Float (single-precision)") (EventReference :type "AnimNotifyEventReference Structure (by ref)"))
  (returns (ReturnValue :type Boolean))
  (`self.SetMeleeTraceEnabled` (`ActorComponent.GetOwner` MeshComp) true)
  (return true))

(fn `Received_NotifyEnd`
  (params (MeshComp :type "SkeletalMeshComponent Object Reference") (Animation :type "AnimSequenceBase Object Reference") (EventReference :type "AnimNotifyEventReference Structure (by ref)"))
  (returns (ReturnValue :type Boolean))
  (bind _meleecomp (`self.SetMeleeTraceEnabled` (`ActorComponent.GetOwner` MeshComp)))
  (`/Game/Defender/Blueprints/Components/MeleeComp.StrikeEnd` _meleecomp)
  (return false))

(fn `SetMeleeTraceEnabled`
  (params (OwnerActor :type "Actor Object Reference") (MeleeTrace :type Boolean))
  (returns (MeleeComp :type "/Game/Defender/Blueprints/Components/MeleeComp Object Reference"))
  (locals (InOwnerActor :type "Actor Object Reference") (InMeleeComp :type "/Game/Defender/Blueprints/Components/MeleeComp Object Reference"))
  (bind _output_get (set `local.InOwnerActor` OwnerActor))
  (bind _output_get_2 (set `local.InMeleeComp` (`Actor.GetComponentByClass` _output_get "/Game/Defender/Blueprints/Components/MeleeComp.MeleeComp_C")))
  (`/Engine/EditorBlueprintResources/StandardMacros.IsValid` _output_get_2
    (:`Is Valid`
      (set `/Game/Defender/Blueprints/Components/MeleeComp.MeleeTraceEnabled` MeleeTrace (`local.InMeleeComp`))
      (return (`local.InMeleeComp`)))))