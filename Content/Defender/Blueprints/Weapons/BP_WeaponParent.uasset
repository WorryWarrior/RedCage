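; Base weapon actor that fires projectiles from the muzzle with random pitch/yaw deflection, shell ejection and sound.
; Magazine ammo is stored per weapon class in the owner's InventoryComp, reserves per projectile type; firing and reloading update both and broadcast ammo changes.
; An optional laser sight traces each tick toward the owner's blackboard TargetActor, steering a beam particle's endpoint.
; Owner death is bound through HealthComp.
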(event `self.ReceiveBeginPlay`
  (set `self.PlayerCharacter` (`GameplayStatics.GetPlayerCharacter` 0))
  (bind _output_get (set `self.OwnerActor` (`self.GetOwner`)))
  (`/Engine/EditorBlueprintResources/StandardMacros.IsValid` _output_get
    (:`Is Valid`
      (bind _output_get_2 (set `self.InventoryComp` (`self.GetComponentByClass` (`self.GetOwner`) "/Game/Defender/Blueprints/Components/InventoryComp.InventoryComp_C")))
      (`/Engine/EditorBlueprintResources/StandardMacros.IsValid` _output_get_2
        (:`Is Valid`
          (add `/Game/Defender/Blueprints/Components/InventoryComp.OnInvAmmoChanged` (`self.InventoryComp`) (delegate `OnInvAmmoChanged_Event_0`))
          (bind _output_get_3 (set `self.HealthComp` (`self.GetComponentByClass` (`self.GetOwner`) "/Game/Defender/Blueprints/Components/HealthComp.HealthComp_C")))
          (add `/Game/Defender/Blueprints/Components/HealthComp.OnDeath` _output_get_3 (`|CreateDelegate` :!event `OnDeath`))
          (if (`self.IsFlashlightVisible`)
            (`SceneComponent.SetVisibility` (`self.FlashLight`) true false)))))))

(event `OnInvAmmoChanged_Event_0`
  (params (Projectile :type "/Game/Defender/Blueprints/Projectiles/BP_ProjectileParent Class Reference") (ChangingAmmo :type Integer) (NewAmmoCount :type Integer))
  (if (== Projectile (`self.Projectile`))
    (`self.OnWeaponAmmoChanged` (`self.GetMagazineAmmo`) (`self.GetInvAmmoCount`))))

(event `self.ReceiveTick`
  (params (DeltaSeconds :type "Float (single-precision)"))
  (`self.LazerSight`))

(event `ActivateLazerSight`
  (set `self.IsLazerSightActivated` true)
  (`/Engine/EditorBlueprintResources/StandardMacros.IsValid` (`self.SniperTrail`)
    (:`Is Not Valid`
      (bind _returnvalue (`GameplayStatics.SpawnEmitterAttached` "/Game/Defender/Demo/Particles/P_SniperTrail.P_SniperTrail" (`self.Muzzle`) "None" (0.0 0.0 0.0) (struct) (0.1 0.1 0.1) "KeepRelativeOffset" false))
      (set `self.SniperTrail` _returnvalue))))

(event `DeactivateLazerSight`
  (bind _snipertrail (`self.SniperTrail`))
  (set `self.IsLazerSightActivated` false)
  (`/Engine/EditorBlueprintResources/StandardMacros.IsValid` _snipertrail
    (:`Is Valid`
      (`ActorComponent.K2_DestroyComponent` _snipertrail))))

(fn `CalculateProjectileRotation`
  (params (TargetLocation :type "Vector Structure"))
  (returns (ReturnValue :type "Rotator Structure"))
  (locals (InTargetLocation :type "Vector Structure"))
  (bind (_return_x _return_y _return_z) (`KismetMathLibrary.BreakVector` (`self.GetDeflection` (`self.DeflectionRate`))))
  (bind (_returnvalue_roll _returnvalue_pitch _returnvalue_yaw) (`KismetMathLibrary.BreakRotator` (`KismetMathLibrary.FindLookAtRotation` (`SceneComponent.K2_GetComponentLocation` (`self.Muzzle`)) (`local.InTargetLocation`))))
  (bind (_returnvalue_roll_2 _returnvalue_pitch_2 _returnvalue_yaw_2) (`KismetMathLibrary.BreakRotator` (`KismetMathLibrary.SelectRotator` (`KismetMathLibrary.MakeRotator` _returnvalue_roll _returnvalue_pitch _returnvalue_yaw) (`KismetMathLibrary.MakeRotator` _returnvalue_roll 0.0 _returnvalue_yaw) (`/Game/Defender/Blueprints/Components/WeaponComp.FiringZActivated` (`self.WeaponComp`)))))
  (set `local.InTargetLocation` TargetLocation)
  (return (`KismetMathLibrary.MakeRotator` (+ _returnvalue_roll_2 _return_x) (+ _returnvalue_pitch_2 _return_y) (+ _returnvalue_yaw_2 _return_z))))

(fn `CanLazerSight`
  (returns (Return :type Boolean))
  (return (and (`self.IsLazerSightActivated`) (`/Game/Defender/Blueprints/Components/HealthComp.isAlive` (`self.HealthComp`)) (`KismetSystemLibrary.IsValid` (`self.SniperTrail`)))))

(fn `Fire`
  (params (TargetLocation :type "Vector Structure"))
  (locals (ProjectileRot :type "Rotator Structure") (InTargetLoc :type "Vector Structure"))
  (set `local.InTargetLoc` TargetLocation) ; Target Location to fire
  (if (> (`self.GetMagazineAmmo`) 0)
    (`self.SetMagazineAmmo` (- (`self.GetMagazineAmmo`) 1))
    (`self.OnWeaponAmmoChanged` (`self.GetMagazineAmmo`) (`self.GetInvAmmoCount`)) ; Ammo Changed Event
    (set `local.ProjectileRot` (`self.CalculateProjectileRotation` (`local.InTargetLoc`)))
    (`|SpawnActorFromClass` (`self.Projectile`) (`KismetMathLibrary.MakeTransform` (`SceneComponent.K2_GetComponentLocation` (`self.Muzzle`)) (`local.ProjectileRot`)) "AdjustIfPossibleButAlwaysSpawn" "SelectDefaultAtRuntime" null null) ; Spawn bullet according to weapon class
    (`GameplayStatics.PlaySoundAtLocation` (`self.FiringSound`) (`self.K2_GetActorLocation`) (struct) 1.0 1.0 0.0 "/Game/Defender/Demo/Audio/Attenuations/ATT_Wep_Shoot.ATT_Wep_Shoot" "/Game/Defender/Demo/Audio/Concurrencies/Con_BulletSound.Con_BulletSound" null null) ; Fire sound
    (`ActorComponent.Activate` (`self.MuzzleParticle`) false)
    (`|SpawnActorFromClass` (`self.ShellEjectClass`) (`SceneComponent.K2_GetComponentToWorld` (`self.ShellEject`)) "AlwaysSpawn" "SelectDefaultAtRuntime" self null)
    (else
      (`/Game/Defender/Blueprints/Components/WeaponComp.OnMagazineEmpty` (`self.WeaponComp`)) ; Weapon magazine empty event dispatcher
      (`GameplayStatics.PlaySoundAtLocation` "/Game/Defender/Demo/Audio/Other/SCue_Launcher_Dryfire.SCue_Launcher_Dryfire" (`self.K2_GetActorLocation`) (struct) 1.0 1.0 0.0 "/Game/Defender/Demo/Audio/Attenuations/ATT_ReloadSound.ATT_ReloadSound" null null null))))

(fn `GetCooldownDelay`
  (returns (ReturnValue :type "Float (double-precision)"))
  (return (/ 1.0 (`KismetMathLibrary.FClamp` (`self.FireRate`) 1.0 10.0))))

(fn `GetDeflection`
  (params (Value :type "Float (double-precision)"))
  (returns (Return :type "Vector Structure"))
  (locals (MapRangedValue :type "Float (double-precision)" :default 0.0))
  (set `local.MapRangedValue` (`KismetMathLibrary.MapRangeClamped` Value 0.0 1.0 0.0 3.0))
  (return (`KismetMathLibrary.MakeVector` 0.0 (`KismetMathLibrary.RandomFloatInRange` (* (`local.MapRangedValue`) -1.0) (`local.MapRangedValue`)) (`KismetMathLibrary.RandomFloatInRange` (* (`local.MapRangedValue`) -1.0) (`local.MapRangedValue`)))) ; Only Pitch and Yaw, not Roll
)

(fn `GetInvAmmoCount`
  (returns (Value :type Integer))
  (return (`/Game/Defender/Blueprints/Components/InventoryComp.GetAmmoCount` (`self.InventoryComp`) (`self.Projectile`))))

(fn `GetMagazineAmmo`
  (returns (Value :type Integer))
  (locals (MagazineCounts :type "Array of  Structure"))
  (bind (_value _returnvalue) (`BlueprintMapLibrary.Map_Find` (`/Game/Defender/Blueprints/Components/InventoryComp.WeaponMagazineAmmoCounts` (`self.InventoryComp`)) (`GameplayStatics.GetObjectClass` self)))
  (`/Engine/EditorBlueprintResources/StandardMacros.IsValid` (`self.InventoryComp`)
    (:`Is Valid`
      (if _returnvalue
        (return _value)
        (else
          (return 0))))
    (:`Is Not Valid`
      (return 0))))

(fn `GetTargetActorBB`
  (returns (AsActor :type "Actor Object Reference"))
  (return (cast `Actor` (`BlackboardComponent.GetValueAsObject` (`AIBlueprintHelperLibrary.GetBlackboard` (`self.OwnerActor`)) "TargetActor") :!pure true)))

(fn `LazerSight`
  (`/Engine/EditorBlueprintResources/StandardMacros.IsValid` (`self.HealthComp`) ; Fix: HealthComp is pending kill
    (:`Is Valid`
      (if (`self.CanLazerSight`)
        (set `self.TargetActor` (`self.GetTargetActorBB`))
        (bind _targetactor (`self.TargetActor`)
          (:`then`
            (bind (_outhit _returnvalue) (`KismetSystemLibrary.LineTraceSingle` (`SceneComponent.K2_GetComponentLocation` (`self.Muzzle`)) (`self.K2_GetActorLocation` _targetactor) "TraceTypeQuery1" true))
            (if _returnvalue
              (set `self.TrailHitActor` (`.HitActor` (`GameplayStatics.BreakHitResult` _outhit)))
              (`self.TrailHitActor`
                (:`then`
                  (set `self.TrailHitActorSK` (`self.GetComponentByClass` (`self.TrailHitActor`) "/Script/Engine.SkeletalMeshComponent"))
                  (bind _trailhitactorsk (`self.TrailHitActorSK`)
                    (:`then`
                      (bind (_returnvalue_x _returnvalue_y _returnvalue_z) (`KismetMathLibrary.BreakVector` (`SceneComponent.K2_GetComponentLocation` _trailhitactorsk)))
                      (`FXSystemComponent.SetVectorParameter` (`self.SniperTrail`) "Target" (`KismetMathLibrary.MakeVector` _returnvalue_x _returnvalue_y (+ _returnvalue_z 100.0))))
                    (:`else`
                      (`FXSystemComponent.SetVectorParameter` (`self.SniperTrail`) "Target" (`self.K2_GetActorLocation` (`self.TrailHitActor`))))))
                (:`else`))
              (else
                (`self.DeactivateLazerSight`))))
          (:`else`))))))

(fn `OnDeath`
  (params (BoneName :type Name) (ShotFromDirection :type "Vector Structure") (HitComponent :type "PrimitiveComponent Object Reference"))
  (`self.DeactivateLazerSight`))

(fn `Reload Completed Actions`
  (locals (EmptyMagazineAmmo :type Integer :default 0) (TotalAmmoPlus :type Integer :default 0))
  (if (> (`self.GetInvAmmoCount`) 0)
    (set `local.EmptyMagazineAmmo` (- (`self.GetMagazineAmmo`) (`self.MagazineSize`)))
    (set `local.TotalAmmoPlus` (+ (`self.GetInvAmmoCount`) (`self.GetMagazineAmmo`)))
    (if (> (- (`local.TotalAmmoPlus`) (`self.MagazineSize`)) 0)
      (`self.SetMagazineAmmo` (`self.MagazineSize`))
      (`self.SetInvAmmoCount` (- (`local.TotalAmmoPlus`) (`self.MagazineSize`)))
      (else
        (`self.SetMagazineAmmo` (`local.TotalAmmoPlus`))
        (`self.SetInvAmmoCount` 0)))
    (`self.OnWeaponAmmoChanged` (`self.GetMagazineAmmo`) (`self.GetInvAmmoCount`))))

(fn `SetInvAmmoCount`
  (params (AmmoCount :type Integer))
  (`/Game/Defender/Blueprints/Components/InventoryComp.SetInvAmmoCount` (`self.InventoryComp`) (`self.Projectile`) AmmoCount))

(fn `SetMagazineAmmo`
  (params (Value :type "Integer (by ref)"))
  (`BlueprintMapLibrary.Map_Add` (`/Game/Defender/Blueprints/Components/InventoryComp.WeaponMagazineAmmoCounts` (`self.InventoryComp`)) (`GameplayStatics.GetObjectClass` self) Value))

(fn `UserConstructionScript`)